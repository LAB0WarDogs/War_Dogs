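; Master AI controller for Puce enemies that runs their behavior tree and drives patrol, investigation and alert states in a stealth setup.
; Sight and hearing perception of the player or dead bodies set Blackboard AIState and target, update the pawn's state and the player's alert UI.
; Sight emits a distance-curve detection speed, while seeing plus hearing triggers full alert.
; Paralysed and Stunned events temporarily halt AI logic, with paralysis also disabling senses.
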(event `AlertDeadBody`
  (params (ActorLocation :type "Vector Structure"))
  (message `/Game/Blueprint/Interface/BPI_ChangeAiStates.ChangeState` (`self.As BP AI Master`) "NewEnumerator2")
  (`BlackboardComponent.SetValueAsEnum` (`self.Blackboard`) "AIState" 1)
  (`BlackboardComponent.SetValueAsVector` (`self.Blackboard`) "TargetLocationVector" ActorLocation)
  (`BlackboardComponent.SetValueAsObject` (`self.Blackboard`) "TargetLocationActor" null)
  (`/Game/Blueprint/Character/CharacterMaster.ResetAlertLevelUI` (`self.CharaMaster`) self)
  (bind _ascharacter_master (cast `/Game/Blueprint/Character/CharacterMaster` (`self.SensedActor`)))
  (`/Game/Blueprint/Character/CharacterMaster.NewAlertState` _ascharacter_master self 1))

(event `PlayerSeen`
  (bind _charamaster (`self.CharaMaster`))
  (bind (_age _expirationage _strength _stimuluslocation _receiverlocation _tag _bsuccessfullysensed) (break `AIStimulus` (`self.AiStimulus`)))
  (`/Engine/EditorBlueprintResources/StandardMacros.IsValid` _charamaster
    (:`Is Valid`
      (`/Game/Blueprint/Character/CharacterMaster.ResetAlertLevelUI` _charamaster self)
      (bind _ascharacter_master (cast `/Game/Blueprint/Character/CharacterMaster` (`self.SensedActor`)))
      (`/Game/Blueprint/Character/CharacterMaster.NewAlertState` _ascharacter_master self 1)
      (`self.SightRegistered` _bsuccessfullysensed (`CurveFloat.GetFloatValue` (`self.SightCurve`) (`KismetMathLibrary.NormalizeToRange` (`KismetMathLibrary.Vector_Distance` _stimuluslocation _receiverlocation) 0.0 1000.0))))))

(event `Alert`
  (bind _as_bp_ai_master (`self.As BP AI Master`))
  (bind _charamaster (`self.CharaMaster`))
  (bind _as_bp_ai_master_2 (`self.As BP AI Master`))
  (if (`self.ActorHasTag` (`self.SensedActor`) "Player") :!label _label
    (if (`.bSuccessfullySensed` (break `AIStimulus` (`self.AiStimulus`)))
      (if (`self.ActorHasTag` (`self.SensedActor`) "Player")
        (set `self.PreviousActorAlerte` false)
        (`/Engine/EditorBlueprintResources/StandardMacros.IsValid` _as_bp_ai_master_2
          (:`Is Valid`
            (message `/Game/Blueprint/Interface/BPI_ChangeAiStates.ChangeState` _as_bp_ai_master_2 "NewEnumerator3")
            (`BlackboardComponent.SetValueAsEnum` (`self.Blackboard`) "AIState" 2)
            (`BlackboardComponent.SetValueAsObject` (`self.Blackboard`) "TargetLocationActor" (`self.SensedActor`))
            (`/Game/Blueprint/Character/CharacterMaster.ResetAlertLevelUI` (`self.CharaMaster`) self)
            (bind _ascharacter_master (cast `/Game/Blueprint/Character/CharacterMaster` (`self.SensedActor`)))
            (`/Game/Blueprint/Character/CharacterMaster.NewAlertState` _ascharacter_master self 2))))
      (else
        (`/Engine/EditorBlueprintResources/StandardMacros.IsValid` _as_bp_ai_master :!label _label_2
          (:`Is Valid`
            (set `self.PreviousActorAlerte` true)
            (message `/Game/Blueprint/Interface/BPI_ChangeAiStates.ChangeState` _as_bp_ai_master "NewEnumerator2")
            (`BlackboardComponent.SetValueAsEnum` (`self.Blackboard`) "AIState" 1)
            (`BlackboardComponent.SetValueAsVector` (`self.Blackboard`) "TargetLocationVector" (`.StimulusLocation` (break `AIStimulus` (`self.AiStimulus`))))
            (`BlackboardComponent.SetValueAsObject` (`self.Blackboard`) "TargetLocationActor" null)
            (`/Engine/EditorBlueprintResources/StandardMacros.IsValid` _charamaster
              (:`Is Valid`
                (`/Game/Blueprint/Character/CharacterMaster.ResetAlertLevelUI` _charamaster self)
                (bind _ascharacter_master_2 (cast `/Game/Blueprint/Character/CharacterMaster` (`self.SensedActor`)))
                (`/Game/Blueprint/Character/CharacterMaster.NewAlertState` _ascharacter_master_2 self 1)))))))
    (else
      (goto _label_2))))

(event `self.AIPerception.OnTargetPerceptionUpdated`
  (params (Actor :type "Actor Object Reference") (Stimulus :type "AIStimulus Structure"))
  (`/Engine/EditorBlueprintResources/StandardMacros.IsValid` Actor
    (:`Is Valid`
      (if (`self.ActorHasTag` Actor "Player")
        (set `self.SensedActor` Actor :!label _label_3)
        (bind _output_get (set `self.AiStimulus` Stimulus))
        (bind _returnvalue (`AIPerceptionSystem.GetSenseClassForStimulus` _output_get))
        (switch `string` (`KismetSystemLibrary.GetClassDisplayName` _returnvalue)
          (:`AISense_Sight`
            (if (`self.ActorHasTag` (`self.SensedActor`) "Player")
              (set `self.AiSeePlayer` true)
              (if (`self.AiHearPlayer`)
                (if (and (`self.AiSeePlayer`) (`self.AiHearPlayer`)) :!label _label_4
                  (goto _label))
                (else
                  (`self.PlayerSeen`)
                  (`BlackboardComponent.SetValueAsVector` (`self.Blackboard`) "TargetLocationVector" (`.StimulusLocation` (break `AIStimulus` (`self.AiStimulus`))))))
              (elif (`self.ActorHasTag` (`self.SensedActor`) "DeadBody")
                (if (not (`|EnumEquality` (`self.AiState`) "NewEnumerator3"))
                  (bind _asbp_puce_dead_body (cast `/Game/Blueprint/Actors/DeadBody/BP_PuceDeadBody` (`self.SensedActor`)))
                  (`/Game/Blueprint/Actors/DeadBody/BP_PuceDeadBody.CheckDeadBody` _asbp_puce_dead_body)
                  (`self.AlertDeadBody` (`/Game/Blueprint/Actors/DeadBody/BP_PuceDeadBody.ActorLocation` _asbp_puce_dead_body))
                  (set `self.AiHearPlayer` true)))))
          (:`AISense_Hearing`
            (if (or (`|EnumEquality` (`self.AiState`) "NewEnumerator1") (`|EnumEquality` (`self.AiState`) "NewEnumerator4") (`|EnumEquality` (`self.AiState`) "NewEnumerator2") (`BlackboardComponent.GetValueAsBool` (`self.Blackboard`) "IsPreInvestigating"))
              (set `self.AiHearPlayer` true)
              (if (`|EnumEquality` (`self.AiState`) "NewEnumerator2")
                (if (`BlackboardComponent.GetValueAsBool` (`self.Blackboard`) "SetTheLoop")
                  (message `/Game/Blueprint/Interface/BPI_ChangeAiStates.ChangeState` (`self.As BP AI Master`) "NewEnumerator5")
                  (`BlackboardComponent.SetValueAsEnum` (`self.Blackboard`) "AIState" 4)
                  (`BlackboardComponent.SetValueAsBool` (`self.Blackboard`) "SetTheLoop" false)
                  (goto _label_2)
                  (else
                    (goto _label_2)))
                (elif (`self.AiSeePlayer`)
                  (goto _label_4)
                  (else
                    (`BlackboardComponent.SetValueAsBool` (`self.Blackboard`) "IsPreInvestigating" false)
                    (message `/Game/Blueprint/Interface/BPI_ChangeAiStates.ChangeState` (`self.As BP AI Master`) "NewEnumerator5")
                    (`BlackboardComponent.SetValueAsEnum` (`self.Blackboard`) "AIState" 4)
                    (`BlackboardComponent.SetValueAsVector` (`self.Blackboard`) "TargetLocationVector" (`.StimulusLocation` (break `AIStimulus` (`self.AiStimulus`))))))))))
        (elif (`self.PreviousActorAlerte`)
          (goto _label_3))))))

(event `self.ReceiveBeginPlay`
  (`self.RunBehaviorTree` (`self.BTAsset`))
  (bind _ascharacter_master (cast `/Game/Blueprint/Character/CharacterMaster` (`GameplayStatics.GetPlayerCharacter` 0)))
  (set `self.CharaMaster` _ascharacter_master)
  (bind _asbp_ai_master (cast `/Game/Blueprint/AI/AI_Puces/AiCharacter/BP_AI_Master` (`self.K2_GetPawn`)))
  (bind _output_get (set `self.As BP AI Master` _asbp_ai_master))
  (`BlackboardComponent.SetValueAsBool` (`AIBlueprintHelperLibrary.GetBlackboard` null) "PathLooping" (`/Game/Blueprint/AI/BP_PatrolPath.IsLooping` (`/Game/Blueprint/AI/AI_Puces/AiCharacter/BP_AI_Master.PatrolPath` _output_get)))
  (`BlackboardComponent.SetValueAsInt` (`AIBlueprintHelperLibrary.GetBlackboard` null) "Direction" 1)
  (`BlackboardComponent.SetValueAsFloat` (`AIBlueprintHelperLibrary.GetBlackboard` null) "WaitTime" (`/Game/Blueprint/AI/BP_PatrolPath.WaitTime` (`/Game/Blueprint/AI/AI_Puces/AiCharacter/BP_AI_Master.PatrolPath` (`self.As BP AI Master`))))
  (`BlackboardComponent.SetValueAsFloat` (`self.Blackboard`) "CheckAngle" (`self.CheckAngle`)))

(event `Paralysed`
  (params (ParalysedTime :type "Float (double-precision)") (`Behavior tree` :type "BehaviorTree Object Reference"))
  (bind _aiperception (`self.AIPerception`))
  (bind _aiperception_2 (`self.AIPerception`))
  (`self.StopMovement`)
  (`BrainComponent.StopLogic` (`self.BrainComponent`) "")
  (`AIPerceptionComponent.SetSenseEnabled` _aiperception_2 "/Script/AIModule.AISense_Sight" false)
  (`AIPerceptionComponent.SetSenseEnabled` _aiperception_2 "/Script/AIModule.AISense_Hearing" false)
  (`KismetSystemLibrary.Delay` ParalysedTime)
  (`self.RunBehaviorTree` `Behavior tree`)
  (`AIPerceptionComponent.SetSenseEnabled` _aiperception "/Script/AIModule.AISense_Sight" true)
  (`AIPerceptionComponent.SetSenseEnabled` _aiperception "/Script/AIModule.AISense_Hearing" true)
  (`self.Alert`))

(event `PreInvestigation`
  (message `/Game/Blueprint/Interface/BPI_ChangeAiStates.ChangeState` (`self.As BP AI Master`) "NewEnumerator5")
  (`BlackboardComponent.SetValueAsEnum` (`self.Blackboard`) "AIState" 4)
  (`BlackboardComponent.SetValueAsVector` (`self.Blackboard`) "TargetLocationVector" (`.StimulusLocation` (break `AIStimulus` (`self.AiStimulus`)))))

(event `Stunned`
  (params (StunnedTime :type "Float (double-precision)"))
  (`self.StopMovement`)
  (`BrainComponent.StopLogic` (`self.BrainComponent`) "")
  (`|PlayMontage` null
    (:`then`
      (`KismetSystemLibrary.Delay` StunnedTime)
      (`BrainComponent.RestartLogic` (`self.BrainComponent`)))))

(event `SeenPlayer`
  (message `/Game/Blueprint/Interface/BPI_ChangeAiStates.ChangeState` (`self.As BP AI Master`) "NewEnumerator4")
  (`BlackboardComponent.SetValueAsEnum` (`self.Blackboard`) "AIState" 3))

(event `SearchPuceKiller`
  (params (Vector3 :type "Vector Structure"))
  (`BlackboardComponent.SetValueAsVector` (`self.Blackboard`) "TargetLocationVector" Vector3))

(event `LostPlayer`
  (message `/Game/Blueprint/Interface/BPI_ChangeAiStates.ChangeState` (`self.As BP AI Master`) "NewEnumerator1")
  (`BlackboardComponent.SetValueAsEnum` (`self.Blackboard`) "AIState" 0)
  (`/Game/Blueprint/Character/CharacterMaster.ResetAlertLevelUI` (`self.CharaMaster`) self))

(fn `HandleSense`
  (params (Selection :type String) (SensedActor :type "Actor Object Reference") (Stimulus :type "AIStimulus Structure"))
  (switch `string` Selection
    (:`AISense_Sight`
      (if (`self.ActorHasTag` (`local.SensedActor`) "Player")
        (`self.PlayerSeen`)))))

(fn `UserConstructionScript`)