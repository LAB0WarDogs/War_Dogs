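; AI flea ("puce") sentinel enemy that leaps at its target character and latches onto them.
; A trigger overlap starts the jump; on contact it forces a switch to the victim if needed, attaches to a random mesh socket and unpossesses itself.
; It then damages nearby damageable actors over time, slows characters and repeatedly reports noise.
; Once the press QTE is flagged complete, it restores speed and replaces itself with a dead body.
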(event `self.ReceiveBeginPlay`
  (`parent.ReceiveBeginPlay`)
  (`self.SpawnDefaultController`)
  (bind _returnvalue (`GameplayStatics.GetActorOfClass` "/Game/Blueprint/WorldMechanics/Relay/BP_RelaySound.BP_RelaySound_C"))
  (`/Engine/EditorBlueprintResources/StandardMacros.IsValid` _returnvalue
    (:`Is Valid`
      (add `/Game/Blueprint/WorldMechanics/Relay/BP_RelaySound.RiseAiMeleeAttackLoudness` _returnvalue (delegate `RiseMeleeLoudness`)))
    (:`Is Not Valid`
      _))
  (bind _asbp_ai_controller_master (cast `/Game/Blueprint/AI/AI_Puces/AIController/BP_AiControllerMaster` (`AIBlueprintHelperLibrary.GetAIController` self)))
  (set `self.As BP Ai Controller Master_0` _asbp_ai_controller_master)
  (`KismetSystemLibrary.K2_SetTimerDelegate` (delegate `CheckIfOnGround`) 0.2 true))

(event `RiseMeleeLoudness`
  (`/Engine/EditorBlueprintResources/StandardMacros.FlipFlop`))

(event `CheckIfOnGround`
  (if (`self.HasToJump`)
    (`KismetSystemLibrary.Delay` 5.0)
    (`BrainComponent.RestartLogic` (`AIController.BrainComponent` (`self.As BP Ai Controller Master_0`)))
    (`PrimitiveComponent.SetSimulatePhysics` (`self.CapsuleComponent`) false)
    (else
      (set `self.JumpSuccess` false))))

(event `/Game/Blueprint/Interface/BPI_ChangeAiStates.ChangeState`
  (params (AlertState :type "/Game/Blueprint/Enum/E_AiStates Enum" :default "NewEnumerator1"))
  (`parent.ChangeState` AlertState))

(event `/Game/Blueprint/Interface/BPI_Damageable.TakeDamage`
  (params (Damage :type "Float (double-precision)"))
  (`parent.TakeDamage` Damage))

(event `ContinueMeleeAttack`
  (bind _returnvalue (`self.GetController`))
  (bind _as_bp_ai_controller_master_0 (`self.As BP Ai Controller Master_0`))
  (`/Game/Blueprint/Character/CharacterMaster.NewPuceAttack` (stale `MeleeAttack` _ascharacter_master) self (`self.PressesNeeded`) :!label _label)
  (set `self.JumpSuccess` false)
  (set `self.IsAttackingPlayer` true)
  (`/Engine/EditorBlueprintResources/StandardMacros.IsValid` _returnvalue
    (:`Is Valid`
      (`Controller.StopMovement` _returnvalue)
      (`PrimitiveComponent.SetCollisionEnabled` (`self.CapsuleComponent`) "NoCollision")
      (`self.K2_AttachToComponent` (`Character.Mesh` (stale `MeleeAttack` _ascharacter_master)) (`KismetArrayLibrary.Array_Random` (`self.SocketNames`)) "SnapToTarget" "SnapToTarget" "KeepWorld" false)
      (`Controller.UnPossess` _returnvalue)
      (`AIPerceptionComponent.SetSenseEnabled` (`/Game/Blueprint/AI/AI_Puces/AIController/BP_AiControllerMaster.AIPerception` _as_bp_ai_controller_master_0) "/Script/AIModule.AISense_Sight" false)
      (`/Game/Blueprint/Character/CharacterMaster.CancelAction` (stale `MeleeAttack` _ascharacter_master))
      (`/Game/Blueprint/Character/CharacterMaster.ResetAlertLevelUI` (stale `MeleeAttack` _ascharacter_master) _as_bp_ai_controller_master_0)
      (`/Game/Blueprint/Character/CharacterMaster.NewAlertState` (stale `MeleeAttack` _ascharacter_master) _as_bp_ai_controller_master_0 2)
      (bind _outactors (`KismetSystemLibrary.SphereOverlapActors` (`self.K2_GetActorLocation`) 250.0 (`self.Object Types`) null (`|MakeArray` self :!type "Actor Object Reference")))
      (for _array_element _outactors
        (if (`KismetSystemLibrary.DoesImplementInterface` _array_element "/Game/Blueprint/Interface/BPI_Damageable.BPI_Damageable_C")
          (set `self.Array Element` _array_element)
          (`self.DamageOverTime`)
          (bind _ascharacter_master (cast `/Game/Blueprint/Character/CharacterMaster` _array_element))
          (bind _output_get (set `self.As Character Master_0` _ascharacter_master))
          (`/Game/Blueprint/Character/CharacterMaster.ReducePlayerSpeed` _output_get)
          (`self.ReportNoise`))))))

(event `MeleeAttack`
  (params (NewParam :type "Actor Object Reference"))
  (`GameplayStatics.PlaySoundAtLocation` "/Game/Sound/Chien/SQ_Jappement.SQ_Jappement" (`self.K2_GetActorLocation`) (struct) 1.0 1.0 0.0 null null null null)
  (`GameplayStatics.PlaySoundAtLocation` "/Game/Sound/Puce/SQ_puce_attaque_Cue.SQ_puce_attaque_Cue" (`self.K2_GetActorLocation`) (struct) 1.0 1.0 0.0 null null null null)
  (bind _ascharacter_master (cast `/Game/Blueprint/Character/CharacterMaster` NewParam))
  (if (not (!= _ascharacter_master (`GameplayStatics.GetPlayerCharacter` 0)))
    (goto _label)
    (else
      (bind _returnvalue (`KismetSystemLibrary.GetDisplayName` _ascharacter_master))
      (`KismetSystemLibrary.PrintString` _returnvalue)
      (switch `string` _returnvalue
        (:`BP_FirstChara_C_0`
          (`self.InCaseFirstCharaIsTargeted`))
        (:`BP_SecondChara_C_0`
          (`self.InCaseSecondCharaIsTargeted`))
        (:`BP_ThirdChara_C_0`
          (`self.InCaseThirdCharaIsTargeted`))))))

(event `DamageOverTime`
  (bind _array_element (`self.Array Element`))
  ;[1 1 1] damage over time + vignette
  (`/Engine/EditorBlueprintResources/StandardMacros.IsValid` _array_element
    (:`Is Valid`
      (message `/Game/Blueprint/Interface/BPI_Damageable.TakeDamage` _array_element 1.0)
      (`KismetSystemLibrary.Delay` 0.1)
      (`self.DamageOverTime`))))

(event `self.Sphere.OnComponentBeginOverlap`
  (params (OverlappedComponent :type "PrimitiveComponent Object Reference") (OtherActor :type "Actor Object Reference") (OtherComp :type "PrimitiveComponent Object Reference") (OtherBodyIndex :type Integer) (bFromSweep :type Boolean) (SweepResult :type "HitResult Structure (by ref)"))
  (bind _ascharacter_master (cast `/Game/Blueprint/Character/CharacterMaster` OtherActor))
  (set `self.JumpSuccess` true)
  (`KismetSystemLibrary.Delay` 0.1)
  (`self.MeleeAttack` _ascharacter_master))

(event `InCaseFirstCharaIsTargeted`
  ;[0 0 1] In case the player caught is not the same as the player controlled, we switch to the player that is being attacked
  (if (`KismetStringLibrary.EqualEqual_StrStr` (`KismetSystemLibrary.GetDisplayName` (`GameplayStatics.GetPlayerCharacter` 0)) "BP_SecondChara_C_0")
    (bind _asgame_mode_wardogs (`/Game/Blueprint/FL_Main.GetGameMode`))
    (set `/Game/Blueprint/GameMode/GameModeWardogs.IsSwitching` true _asgame_mode_wardogs)
    (`/Game/Blueprint/GameMode/GameModeWardogs.SwitchChara1` _asgame_mode_wardogs)
    (else
      (bind _asgame_mode_wardogs_2 (`/Game/Blueprint/FL_Main.GetGameMode`))
      (set `/Game/Blueprint/GameMode/GameModeWardogs.IsSwitching` true _asgame_mode_wardogs_2)
      (`/Game/Blueprint/GameMode/GameModeWardogs.SwitchChara0` _asgame_mode_wardogs_2)))
  (`self.ContinueMeleeAttack`))

(event `ReportNoise`
  (bind _as_character_master_0 (`self.As Character Master_0`))
  (if (not (`self.QTeIsComplete`))
    (`AISense_Hearing.ReportNoiseEvent` (`self.K2_GetActorLocation`) 1.0 (`self.As Character Master_0`) 2000.0)
    (`KismetSystemLibrary.Delay` 0.1)
    (`self.ReportNoise`)
    (else
      (bind _asmy_player_controller (`/Game/Blueprint/FL_Main.GetPlayerController`))
      (set `/Game/Blueprint/Character/MyPlayerController.IsBeingAttack` false _asmy_player_controller)
      (`/Game/Blueprint/Character/CharacterMaster.RestorePlayerSpeed` _as_character_master_0)
      (`/Game/Blueprint/Character/CharacterMaster.ResetAlertLevelUI` _as_character_master_0 (`self.As BP Ai Controller Master_0`))
      (`self.K2_DetachFromActor` "KeepWorld")
      (bind _returnvalue (`|SpawnActorFromClass` "/Game/Blueprint/Actors/DeadBody/BP_PuceDeadBody.BP_PuceDeadBody_C" (`self.GetTransform` self) "Undefined" "OverrideRootScale" null null))
      (`/Game/Blueprint/Actors/DeadBody/BP_PuceDeadBody.InitializationDeadBody` _returnvalue (`self.K2_GetActorLocation` (`GameplayStatics.GetPlayerController` 0)) self)
      (set `self.IsAttackingPlayer` false)
      (`self.K2_DestroyActor`))))

(event `/Game/Blueprint/Interface/BPI_InteractWithEnnemy.InteractWithEnnemy`
  ;[0 1 0] desactiver pour les test
)

(event `InCaseSecondCharaIsTargeted`
  ;[0 0 1] In case the player caught is not the same as the player controlled, we switch to the player that is being attacked
  (if (`KismetStringLibrary.EqualEqual_StrStr` (`KismetSystemLibrary.GetDisplayName` (`GameplayStatics.GetPlayerCharacter` 0)) "BP_FirstChara_C_0")
    (bind _asgame_mode_wardogs (`/Game/Blueprint/FL_Main.GetGameMode`))
    (set `/Game/Blueprint/GameMode/GameModeWardogs.IsSwitching` true _asgame_mode_wardogs)
    (`/Game/Blueprint/GameMode/GameModeWardogs.SwitchChara0` _asgame_mode_wardogs)
    (else
      (bind _asgame_mode_wardogs_2 (`/Game/Blueprint/FL_Main.GetGameMode`))
      (set `/Game/Blueprint/GameMode/GameModeWardogs.IsSwitching` true _asgame_mode_wardogs_2)
      (`/Game/Blueprint/GameMode/GameModeWardogs.SwitchChara1` _asgame_mode_wardogs_2)))
  (`self.ContinueMeleeAttack`))

(event `/Game/Blueprint/Interface/BPI_InteractWithEnnemy.StopInteractWithEnnemy`
  ;[0 1 0] desactiver pour les test
)

(event `DecrementProgressBar`
  (bind _widgetref (`self.WidgetRef`))
  (bind _pressedamount (`self.PressedAmount`))
  ;[0 1 0] desactiver pour les test
  (bind _result (`/Engine/EditorBlueprintResources/StandardMacros.DecrementFloat` _pressedamount)
    (:`  `
      (bind _output_get (set `self.PressedAmount` (`KismetMathLibrary.FClamp` _result 0.0 _pressedamount)))
      (`/Engine/EditorBlueprintResources/StandardMacros.IsValid` _widgetref
        (:`Is Valid`
          (set `/Game/UI/SpamE/W_SpamE.AmountPressed` _output_get _widgetref)
          (if (<= (`self.PressedAmount`) 0.0)
            (`KismetSystemLibrary.K2_ClearAndInvalidateTimerHandle` (`self.TimerDecrementProgressBarRef`))))))))

(event `InCaseThirdCharaIsTargeted`
  ;[0 0 1] In case the player caught is not the same as the player controlled, we switch to the player that is being attacked
  (if (`KismetStringLibrary.EqualEqual_StrStr` (`KismetSystemLibrary.GetDisplayName` (`GameplayStatics.GetPlayerCharacter` 0)) "BP_FirstChara_C_0")
    (bind _asgame_mode_wardogs (`/Game/Blueprint/FL_Main.GetGameMode`))
    (set `/Game/Blueprint/GameMode/GameModeWardogs.IsSwitching` true _asgame_mode_wardogs)
    (`/Game/Blueprint/GameMode/GameModeWardogs.SwitchChara1` _asgame_mode_wardogs)
    (else
      (bind _asgame_mode_wardogs_2 (`/Game/Blueprint/FL_Main.GetGameMode`))
      (set `/Game/Blueprint/GameMode/GameModeWardogs.IsSwitching` true _asgame_mode_wardogs_2)
      (`/Game/Blueprint/GameMode/GameModeWardogs.SwitchChara0` _asgame_mode_wardogs_2)))
  (`self.ContinueMeleeAttack`))

(event `RotateAiWhileInResearchMode`
  (params (RotationAngle :type "Float (double-precision)"))
  (bind (_returnvalue_roll _returnvalue_pitch _returnvalue_yaw) (`KismetMathLibrary.BreakRotator` (`self.K2_GetActorRotation`)))
  (bind _return_value_z__yaw_ (`self.Return Value Z (Yaw)`))
  (set `self.Rotation Angle` RotationAngle)
  (set `self.Return Value Z (Yaw)` _returnvalue_yaw)
  (`TimelineComponent.SetPlayRate` (`self.Timeline`) (/ 1.0 1.0))
  (bind (_direction _airotation) (`Timeline|Timeline` :!via `PlayFromStart`)
    (:`Update`
      (`self.K2_SetActorRotation` (`KismetMathLibrary.MakeRotator` 0.0 0.0 (`KismetMathLibrary.Lerp` _return_value_z__yaw_ (+ _return_value_z__yaw_ (`self.Rotation Angle`)) _airotation))))
    (:`Finished`
      (set `self.Rotation Angle` 0.0))))

(event `self.CollisionJumpStart.OnComponentBeginOverlap`
  (params (OverlappedComponent :type "PrimitiveComponent Object Reference") (OtherActor :type "Actor Object Reference") (OtherComp :type "PrimitiveComponent Object Reference") (OtherBodyIndex :type Integer) (bFromSweep :type Boolean) (SweepResult :type "HitResult Structure (by ref)"))
  (bind _detectedactorarray (`self.DetectedActorArray`))
  (bind _ascharacter_master (cast `/Game/Blueprint/Character/CharacterMaster` OtherActor))
  (`KismetArrayLibrary.Array_AddUnique` _detectedactorarray _ascharacter_master)
  (for _array_element _detectedactorarray
    (if (== _array_element (`BlackboardComponent.GetValueAsObject` (`AIController.Blackboard` (`self.As BP Ai Controller Master_0`)) "TargetLocationActor"))
      (set `self.HasToJump` true)
      (`self.Jump`)
      (`KismetSystemLibrary.Delay` 0.5)
      (set `self.HasToJump` false)
      (`KismetArrayLibrary.Array_Clear` (`self.DetectedActorArray`)))))

(event `self.CollisionJumpStart.OnComponentEndOverlap`
  (params (OverlappedComponent :type "PrimitiveComponent Object Reference") (OtherActor :type "Actor Object Reference") (OtherComp :type "PrimitiveComponent Object Reference") (OtherBodyIndex :type Integer))
  (bind _ascharacter_master (cast `/Game/Blueprint/Character/CharacterMaster` OtherActor))
  (`KismetArrayLibrary.Array_RemoveItem` (`self.DetectedActorArray`) _ascharacter_master)
  (if (<= (`KismetArrayLibrary.Array_Length` (`self.DetectedActorArray`)) 0)
    (`KismetArrayLibrary.Array_Clear` (`self.DetectedActorArray`))))

(fn `UserConstructionScript`
  (`parent.UserConstructionScript`))