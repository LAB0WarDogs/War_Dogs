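; Master AI character for the "Puce" enemies, handling alert-state feedback, health and death.
; ChangeState sets walk speed and detected/research widget visibility per alert state, clearing the AI controller's see/hear flags on Neutral.
; Lethal damage resets the player's alert UI, spawns and initializes a BP_PuceDeadBody, then destroys the actor.
; A retriggerable delay hides the trace Niagara effect and custom-depth outline.
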(event `self.ReceiveBeginPlay`
  (`|ExecutionSequence`
    (:`then_0`
      (bind _foundwidgets (`WidgetBlueprintLibrary.GetAllWidgetsOfClass` "/Game/UI/UI_InGame/Widget_HeadUp.Widget_HeadUp_C" false))
      (set `self.W_HeadUpRef` (`|GetArrayItem` _foundwidgets))
      (bind _ascharacter_master (cast `/Game/Blueprint/Character/CharacterMaster` (`GameplayStatics.GetPlayerCharacter` 0)))
      (set `self.As Character Master` _ascharacter_master)
      (bind _asbp_ai_controller_master (cast `/Game/Blueprint/AI/AI_Puces/AIController/BP_AiControllerMaster` (`AIBlueprintHelperLibrary.GetAIController` self)))
      (set `self.As BP Ai Controller Master` _asbp_ai_controller_master))
    (:`then_1`
      (bind _asw_detection_ai (cast `/Game/UI/UI_InGame/Ui_DetectionAI/W_DetectionAI` (`WidgetComponent.GetUserWidgetObject` (`self.DetectionWidget`))))
      (set `/Game/UI/UI_InGame/Ui_DetectionAI/W_DetectionAI.PawnOwner` self _asw_detection_ai))))

(event `/Game/Blueprint/Interface/BPI_ChangeAiStates.ChangeState`
  (params (AlertState :type "/Game/Blueprint/Enum/E_AiStates Enum" :default "NewEnumerator1"))
  (bind _as_bp_ai_controller_master (`self.As BP Ai Controller Master`))
  (set `self.Alert State` AlertState)
  (`/Engine/EditorBlueprintResources/StandardMacros.DoOnce` false :!label _label
    (:`Completed`
      (set `CharacterMovementComponent.MaxWalkSpeed` (select `/Game/Blueprint/Enum/E_AiStates` (`self.Alert State`) :`NewEnumerator1` 350.0 :`NewEnumerator2` 400.0 :`NewEnumerator3` 650.0 :`NewEnumerator4` 100.0 :`NewEnumerator5` 300.0) (`self.CharacterMovement`))
      (switch `/Game/Blueprint/Enum/E_AiStates` (`self.Alert State`)
        (:`NewEnumerator1`
          (set `/Game/Blueprint/AI/AI_Puces/AIController/BP_AiControllerMaster.AiHearPlayer` false _as_bp_ai_controller_master)
          (set `/Game/Blueprint/AI/AI_Puces/AIController/BP_AiControllerMaster.AiSeePlayer` false _as_bp_ai_controller_master)
          (`self.SetWidgetVisibility` false))
        (:`NewEnumerator2`
          (`self.SetWidgetVisibility` false true :!label _label_2))
        (:`NewEnumerator3`
          (`self.SetWidgetVisibility` true))
        (:`NewEnumerator4`
          (goto _label_2))
        (:`NewEnumerator5`
          (goto _label_2)))
      (`self.ResetAlert`))))

(event `ResetAlert`
  (goto _label :!via `Reset`))

(event `/Game/Blueprint/Interface/BPI_Damageable.TakeDamage`
  (params (Damage :type "Float (double-precision)"))
  (`self.AiTakeDamage` Damage)
  (if (<= (`self.Health`) 0.0)
    (`KismetSystemLibrary.Delay` 0.1)
    (`/Game/Blueprint/Character/CharacterMaster.ResetAlertLevelUI` (`self.As Character Master`) (`self.As BP Ai Controller Master`))
    (`self.K2_DestroyActor`)))

(event `HIdeOutlineAndVFX`
  (`KismetSystemLibrary.RetriggerableDelay` 10.0)
  (`SceneComponent.SetHiddenInGame` (`self.NS_TempoPuceTrace`) true false)
  (`PrimitiveComponent.SetRenderCustomDepth` (`self.Mesh`) false))

(fn `AiTakeDamage`
  (params (DamageTaken :type "Float (double-precision)"))
  (bind _output_get (set `self.Health` (- (`self.Health`) DamageTaken)))
  (`KismetSystemLibrary.PrintString` (`KismetStringLibrary.Concat_StrStr` "AI health is " (`KismetStringLibrary.Conv_DoubleToString` _output_get)))
  (if (<= (`self.Health`) 0.0)
    (`/Game/Blueprint/Character/CharacterMaster.ResetAlertLevelUI` (`self.As Character Master`) (`self.As BP Ai Controller Master`))
    (bind _returnvalue (`|SpawnActorFromClass` "/Game/Blueprint/Actors/DeadBody/BP_PuceDeadBody.BP_PuceDeadBody_C" (`self.GetTransform` self) "Undefined" "OverrideRootScale" null null))
    (`/Game/Blueprint/Actors/DeadBody/BP_PuceDeadBody.InitializationDeadBody` _returnvalue (`self.K2_GetActorLocation` (`GameplayStatics.GetPlayerController` 0)) self)))

(fn `UserConstructionScript`)