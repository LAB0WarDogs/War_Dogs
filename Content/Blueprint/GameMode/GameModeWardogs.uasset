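; Game mode for a game with three switchable characters, handling spawning, switching, HUD and end-game screen.
; BeginPlay loads or creates the save, applies per-level start settings and spawns all three, placing unavailable ones at a trash transform; EndPlay saves.
; Switch events cycle playable characters, cancel actions and call PossesChara, which blends the camera before possessing and restores the previous character's default controller.
; A looping timer shows the end-game widget once any character leaves the list.
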(event `SwitchChara0`
  ;[0 0 1] Switch Character
  (if (and (`self.CanSwitch`) (`self.IsSwitching`))
    (bind _ascharacter_master (cast `/Game/Blueprint/Character/CharacterMaster` (`GameplayStatics.GetPlayerCharacter` 0)))
    (set `self.camRotate` (`/Game/Blueprint/Character/CharacterMaster.CamRotation` _ascharacter_master))
    (`|ExecutionSequence`
      (:`then_0`
        (bind _output_get (set `self.CharaIndex` (+ (`self.CharaIndex`) 1)))
        (if (> _output_get (- (`KismetArrayLibrary.Array_Length` (`self.ArrayCharaRef`)) (+ (`self.CharraNonePlayed`) 1)))
          (set `self.CharaIndex` 0))
        (bind _aspawn (cast `Pawn` (`|GetArrayItem` (`self.ArrayCharaRef`) (`self.CharaIndex`))))
        (bind _ascharacter_master_2 (cast `/Game/Blueprint/Character/CharacterMaster` _aspawn))
        (set `/Game/Blueprint/Character/CharacterMaster.ForcedCrouched` false _ascharacter_master_2)
        ;[0 1 0] Call Ui SwhichChara
        (`/Game/UI/UI_InGame/Widget_HeadUp.Switch` (`self.InGameUI`) (`self.CharaIndex`) (`/Game/Blueprint/Character/CharacterMaster.CanUseFirstSkill` _ascharacter_master_2) (`/Game/Blueprint/Character/CharacterMaster.CanUseSecondarySkill` _ascharacter_master_2) (`/Game/Blueprint/Character/CharacterMaster.CanUseThirdSkill` _ascharacter_master_2))
        (`self.PossesChara` _aspawn)
        (`self.CharacterAsBeenSwitched`)
        (set `self.IsSwitching` false))
      (:`then_1`
        (for _array_element (`self.ArrayCharaRef`)
          (bind _ascharacter_master_3 (cast `/Game/Blueprint/Character/CharacterMaster` _array_element))
          (`/Game/Blueprint/Character/CharacterMaster.CancelAction` _ascharacter_master_3))))))

(event `SwitchChara1`
  ;[0 0 1] Switch Character
  (if (and (`self.CanSwitch`) (`self.IsSwitching`))
    (bind _ascharacter_master (cast `/Game/Blueprint/Character/CharacterMaster` (`GameplayStatics.GetPlayerCharacter` 0)))
    (set `self.camRotate` (`/Game/Blueprint/Character/CharacterMaster.CamRotation` _ascharacter_master))
    (`|ExecutionSequence`
      (:`then_0`
        (bind _output_get (set `self.CharaIndex` (- (`self.CharaIndex`) 1)))
        (if (< _output_get 0)
          (set `self.CharaIndex` (- (`KismetArrayLibrary.Array_Length` (`self.ArrayCharaRef`)) (+ (`self.CharraNonePlayed`) 1))))
        (bind _aspawn (cast `Pawn` (`|GetArrayItem` (`self.ArrayCharaRef`) (`self.CharaIndex`))))
        (bind _ascharacter_master_2 (cast `/Game/Blueprint/Character/CharacterMaster` _aspawn))
        (set `/Game/Blueprint/Character/CharacterMaster.ForcedCrouched` false _ascharacter_master_2)
        ;[0 1 0] Call Ui SwhichChara
        (`/Game/UI/UI_InGame/Widget_HeadUp.Switch` (`self.InGameUI`) (`self.CharaIndex`) (`/Game/Blueprint/Character/CharacterMaster.CanUseFirstSkill` _ascharacter_master_2) (`/Game/Blueprint/Character/CharacterMaster.CanUseSecondarySkill` _ascharacter_master_2) (`/Game/Blueprint/Character/CharacterMaster.CanUseThirdSkill` _ascharacter_master_2))
        (`self.PossesChara` _aspawn)
        (`self.CharacterAsBeenSwitched`)
        (set `self.IsSwitching` false))
      (:`then_1`
        (for _array_element (`self.ArrayCharaRef`)
          (bind _ascharacter_master_3 (cast `/Game/Blueprint/Character/CharacterMaster` _array_element))
          (`/Game/Blueprint/Character/CharacterMaster.CancelAction` _ascharacter_master_3))))))

(event `RemoveFromPlayerList`
  (params (CharaRef :type "Actor Object Reference"))
  (bind _arraychararef (`self.ArrayCharaRef`))
  ;[0 0 1] Remove From Player List
  (`KismetArrayLibrary.Array_RemoveItem` _arraychararef CharaRef)
  (`KismetSystemLibrary.PrintString` (`KismetStringLibrary.Concat_StrStr` "number of player left " (`KismetStringLibrary.Conv_IntToString` (`KismetArrayLibrary.Array_Length` _arraychararef)))))

(event `self.ReceiveBeginPlay`
  (bind _arraychararef (`self.ArrayCharaRef`))
  (bind (_spawntransform_location _spawntransform_rotation _spawntransform_scale) (`KismetMathLibrary.BreakTransform` (`self.SpawnTransform`)))
  (bind (_spawntransform_location_2 _spawntransform_rotation_2 _spawntransform_scale_2) (`KismetMathLibrary.BreakTransform` (`self.SpawnTransform`)))
  (bind _as_bp_save_game (`self.As BP Save Game`))
  (bind _lastplayerselected (`self.LastPlayerSelected`))
  (bind _ingameui (`self.InGameUI`))
  (bind _skillisactive (`self.skillIsActive`))
  ;[0 0 1] Begin Play
  (`|ExecutionSequence`
    (:`then_0`
      (bind _returnvalue (`GameplayStatics.DoesSaveGameExist` "save1"))
      (`KismetSystemLibrary.PrintString` (`KismetStringLibrary.Conv_BoolToString` _returnvalue))
      (if (not _returnvalue)
        (bind _returnvalue_2 (`GameplayStatics.CreateSaveGameObject` "/Game/Blueprint/BP_SaveGame.BP_SaveGame_C"))
        (`GameplayStatics.SaveGameToSlot` _returnvalue_2 "save1"))
      (bind _returnvalue_3 (`GameplayStatics.LoadGameFromSlot` "save1"))
      (bind _asbp_save_game (cast `/Game/Blueprint/BP_SaveGame` _returnvalue_3))
      (set `self.As BP Save Game` _asbp_save_game)
      (bind _returnvalue_4 (`GameplayStatics.GetCurrentLevelName` true))
      (if (`KismetStringLibrary.EqualEqual_StrStr` _returnvalue_4 (`/Game/Blueprint/BP_SaveGame.Level` (`self.As BP Save Game`)))
        (bind _output_get (set `self.CharraNonePlayed` (- 3 (`/Game/Blueprint/BP_SaveGame.CharraInGame` (`self.As BP Save Game`)))))
        (if (== _output_get 2)
          (set `self.CanSwitch` false)
          (else
            (set `self.CanSwitch` true)))
        (else
          (set `/Game/Blueprint/BP_SaveGame.Level` _returnvalue_4 (`self.As BP Save Game`))
          (if (`KismetStringLibrary.EqualEqual_StrStr` (`/Game/Blueprint/BP_SaveGame.Level` (`self.As BP Save Game`)) "LEVEL")
            (set `/Game/Blueprint/BP_SaveGame.PlayerPos` (`self.StartingPosLEVEL`) (`self.As BP Save Game`))
            (set `/Game/Blueprint/BP_SaveGame.CharraInGame` 1 (`self.As BP Save Game`))
            (set `self.CanSwitch` false)
            (set `self.skillIsActive` false)
            (set `self.CharraNonePlayed` 2)
            (else
              (if (`KismetStringLibrary.EqualEqual_StrStr` (`/Game/Blueprint/BP_SaveGame.Level` (`self.As BP Save Game`)) "Map_IntroSuite")
                (set `/Game/Blueprint/BP_SaveGame.PlayerPos` (`self.StartingPosMapIntroSuite`) (`self.As BP Save Game`))
                (bind _output_get_2 (set `/Game/Blueprint/BP_SaveGame.CharraInGame` 1 (`self.As BP Save Game`)))
                (set `self.CanSwitch` false)
                (set `self.CharraNonePlayed` (- 3 _output_get_2) :!label _label)
                (elif (`KismetStringLibrary.EqualEqual_StrStr` (`/Game/Blueprint/BP_SaveGame.Level` (`self.As BP Save Game`)) "MapAssembler")
                  (set `/Game/Blueprint/BP_SaveGame.PlayerPos` (`self.StartingPosMapAssembler`) (`self.As BP Save Game`))
                  (set `/Game/Blueprint/BP_SaveGame.CharraInGame` 1 (`self.As BP Save Game`))
                  (set `self.CanSwitch` false)
                  (goto _label)
                  (else
                    (set `/Game/Blueprint/BP_SaveGame.PlayerPos` (`KismetMathLibrary.MakeTransform` (-310.0 1485.0 148.0)) _as_bp_save_game)
                    (bind _output_get_3 (set `/Game/Blueprint/BP_SaveGame.CharraInGame` 3 _as_bp_save_game))
                    (set `self.CanSwitch` true)
                    (set `self.CharraNonePlayed` (- 3 _output_get_3)))))
              (set `self.skillIsActive` true)))))
      (set `self.SpawnTransform` (`/Game/Blueprint/BP_SaveGame.PlayerPos` (`self.As BP Save Game`)))
      (for _array_element _arraychararef
        (`self.K2_DestroyActor` _array_element))
      (`KismetArrayLibrary.Array_Clear` _arraychararef)
      (`|ExecutionSequence`
        (:`then_0`
          (bind _returnvalue_5 (`|SpawnActorFromClass` "/Game/Blueprint/Character/BP_FirstChara.BP_FirstChara_C" (`self.SpawnTransform`) "Undefined" "OverrideRootScale" null null))
          (`Controller.Possess` (`GameplayStatics.GetPlayerController` 0) _returnvalue_5)
          (`KismetArrayLibrary.Array_AddUnique` (`self.ArrayCharaRef`) _returnvalue_5))
        (:`then_1`
          (if (not (> (`/Game/Blueprint/BP_SaveGame.CharraInGame` (`self.As BP Save Game`)) 1))
            (set `self.SpawnTransform` (`self.TrashTransform`)))
          (bind _returnvalue_6 (`|SpawnActorFromClass` "/Game/Blueprint/Character/BP_SecondChara.BP_SecondChara_C" (`KismetMathLibrary.MakeTransform` (+ _spawntransform_location_2 (150.0 0.0 0.0)) _spawntransform_rotation_2 _spawntransform_scale_2) "Undefined" "OverrideRootScale" null null))
          (`KismetArrayLibrary.Array_AddUnique` (`self.ArrayCharaRef`) _returnvalue_6))
        (:`then_2`
          (if (not (> (`/Game/Blueprint/BP_SaveGame.CharraInGame` (`self.As BP Save Game`)) 2))
            (set `self.SpawnTransform` (`self.TrashTransform`)))
          (bind _returnvalue_7 (`|SpawnActorFromClass` "/Game/Blueprint/Character/BP_ThirdChara.BP_ThirdChara_C" (`KismetMathLibrary.MakeTransform` (+ _spawntransform_location (-150.0 0.0 0.0)) _spawntransform_rotation _spawntransform_scale) "Undefined" "OverrideRootScale" null null))
          (`KismetArrayLibrary.Array_AddUnique` (`self.ArrayCharaRef`) _returnvalue_7)
          (bind _output_get_4 (set `self.LastPlayerSelected` (`|GetArrayItem` (`self.ArrayCharaRef`))))
          (`KismetSystemLibrary.PrintString` (`KismetSystemLibrary.GetDisplayName` _output_get_4))
          (if (not (`self.skillIsActive`))
            (bind _ascharacter_master (cast `/Game/Blueprint/Character/CharacterMaster` _lastplayerselected))
            (set `/Game/Blueprint/Character/CharacterMaster.CanUseFirstSkill` false _ascharacter_master)
            (set `/Game/Blueprint/Character/CharacterMaster.CanUseSecondarySkill` false _ascharacter_master)
            (set `/Game/Blueprint/Character/CharacterMaster.CanUseThirdSkill` false _ascharacter_master)
            (else
              (bind _ascharacter_master_2 (cast `/Game/Blueprint/Character/CharacterMaster` _lastplayerselected))
              (set `/Game/Blueprint/Character/CharacterMaster.CanUseFirstSkill` true _ascharacter_master_2)
              (set `/Game/Blueprint/Character/CharacterMaster.CanUseSecondarySkill` true _ascharacter_master_2)
              (set `/Game/Blueprint/Character/CharacterMaster.CanUseThirdSkill` true _ascharacter_master_2))))))
    (:`then_1`
      ;;[0 1 0] Set HeadUpDisplay
      (bind _returnvalue_8 (`|CreateWidget` "/Game/UI/Dialogue/HeadUpDisplay.HeadUpDisplay_C"))
      (bind _output_get_5 (set `self.HeadUpDisplay` _returnvalue_8))
      (`UserWidget.AddToViewport` _output_get_5 0)
      (bind _returnvalue_9 (`|CreateWidget` "/Game/UI/UI_InGame/Widget_HeadUp.Widget_HeadUp_C"))
      (bind _output_get_6 (set `self.InGameUI` _returnvalue_9))
      (`UserWidget.AddToViewport` _output_get_6 0)
      (`/Game/UI/UI_InGame/Widget_HeadUp.Switch` _ingameui (`self.CharaIndex`) _skillisactive _skillisactive _skillisactive)
      (`/Game/UI/UI_InGame/Widget_HeadUp.SetActiveChara` _ingameui (`/Game/Blueprint/BP_SaveGame.CharraInGame` (`self.As BP Save Game`))))
    (:`then_2`
      (`KismetSystemLibrary.K2_SetTimerDelegate` (delegate `ResetScene`) 0.5 true))
    (:`then_3`
      (`|SpawnActorFromClass` "/Game/Blueprint/Character/BP_ShootCamera.BP_ShootCamera_C" (`KismetMathLibrary.MakeTransform` (0.0 0.0 0.0)) "Undefined" "OverrideRootScale" null null)
      (`|SpawnActorFromClass` "/Game/Blueprint/Actors/DissolveMask/BP_DissolveMask.BP_DissolveMask_C" (`KismetMathLibrary.MakeTransform` (0.0 0.0 0.0) (struct) (10.0 10.0 10.0)) "Undefined" "OverrideRootScale" null null))))

(event `self.ReceiveEndPlay`
  (params (EndPlayReason :type "EEndPlayReason Enum" :default "Destroyed"))
  (`GameplayStatics.SaveGameToSlot` (`self.As BP Save Game`) "save1"))

(event `ResetScene`
  (bind _returnvalue (`GameplayStatics.GetPlayerController` 0))
  ;[0 0 1] Begin Play
  (if (<= (`KismetArrayLibrary.Array_Length` (`self.ArrayCharaRef`)) 2)
    (`/Engine/EditorBlueprintResources/StandardMacros.DoOnce` false :!label _label_2
      (:`Completed`
        (`KismetSystemLibrary.Delay` 3.0)
        (bind _returnvalue_2 (`|CreateWidget` "/Game/UI/UI_Unique/W_EndGame.W_EndGame_C"))
        (`UserWidget.AddToViewport` _returnvalue_2 0)
        (set `PlayerController.bShowMouseCursor` true _returnvalue)
        (`WidgetBlueprintLibrary.SetInputMode_UIOnlyEx` _returnvalue null)))))

(event `ResetDoOnce`
  ;[0 0 1] Begin Play
  (goto _label_2 :!via `Reset`))

(fn `UserConstructionScript`)