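; Destructible wall actor that shatters when it takes environment damage.
; The damage event hides the intact static mesh, disables its collision and reveals the destructible mesh in its place.
; It then applies the incoming damage at that mesh's world location, using impulse direction and strength variables stored on the Blueprint.
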(event `/Game/Blueprint/Interface/BPI_Damageable.EnvironmentTakingDamage`
  (params (Damage :type "Float (double-precision)"))
  (bind _editorcube_dm (`self.EditorCube_DM`))
  (bind _staticmesh (`self.StaticMesh`))
  (`SceneComponent.SetVisibility` _staticmesh false false)
  (`PrimitiveComponent.SetCollisionEnabled` _staticmesh "NoCollision")
  (`SceneComponent.SetVisibility` (`self.EditorCube_DM`) true false)
  (`DestructibleComponent.ApplyDamage` _editorcube_dm Damage (`SceneComponent.K2_GetComponentLocation` _editorcube_dm) (`KismetMathLibrary.MakeVector` (`self.Impulse Dir X`) (`self.Impulse Dir Y`)) (`self.Impulse Strength`)))

(fn `UserConstructionScript`)