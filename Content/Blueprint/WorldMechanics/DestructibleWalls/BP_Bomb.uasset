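; BP_Bomb is a bomb for destructible walls that uses physics fields to break and scatter Chaos destruction pieces.
; Its Explode event applies a radial external cluster strain with no falloff inside the Sphere component's scaled radius, fracturing clusters.
; It then applies a radial linear velocity from the sphere's center, using a culling field to confine the push to that same radius.
; The file contains no trigger for Explode.
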(event `Explode`
  (bind _sphere (`self.Sphere`))
  (bind _returnvalue (`RadialFalloff.SetRadialFalloff` (`self.RadialFalloff`) 500000.0 0.0 1.0 0.0 (`SphereComponent.GetScaledSphereRadius` _sphere) (`SceneComponent.K2_GetComponentLocation` _sphere) "Field_FallOff_None"))
  (`FieldSystemComponent.ApplyPhysicsField` (`self.FieldSystemComponent`) true "Field_ExternalClusterStrain" null _returnvalue)
  (`FieldSystemComponent.ApplyPhysicsField` (`self.FieldSystemComponent`) true "Field_LinearVelocity" null (`CullingField.SetCullingField` (`self.CullingField`) _returnvalue (`RadialVector.SetRadialVector` (`self.RadialVector`) 500.0 (`SceneComponent.K2_GetComponentLocation` (`self.Sphere`))) "Field_Culling_Outside")))

(fn `UserConstructionScript`)