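; BP_ShootCamera is a camera actor that attaches to the first-person character and stays aimed at its SniperCompTarget component.
; On BeginPlay it finds BP_FirstChara, snaps to its Arrow1 and starts a looping timer that turns the camera with FindLookAtRotation, rather than using Tick.
; The game mode's OnRespawn event re-runs this whole setup, including the timer and the binding.
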(event `self.ReceiveBeginPlay`
  (`|ExecutionSequence` :!label _label
    (:`then_0`
      (bind _returnvalue (`GameplayStatics.GetActorOfClass` "/Game/Blueprint/Character/BP_FirstChara.BP_FirstChara_C"))
      (bind _output_get (set `self.FirstCharaRef` _returnvalue))
      (`self.K2_AttachToComponent` (`/Game/Blueprint/Character/BP_FirstChara.Arrow1` _output_get) "None" "SnapToTarget" "KeepRelative" "KeepRelative" false)
      (`KismetSystemLibrary.K2_SetTimerDelegate` (delegate `ChangeCamRot`) 0.1 true))
    (:`then_1`
      (bind _asgame_mode_wardogs (`/Game/Blueprint/FL_Main.GetGameMode`))
      (add `/Game/Blueprint/GameMode/GameModeWardogs.OnRespawn` _asgame_mode_wardogs (delegate `ResetSpecs`)))))

(event `ChangeCamRot`
  (`self.SetCamRot`))

(event `ResetSpecs`
  (goto _label))

(event `SetCamRot`
  (bind _camera (`self.Camera`))
  (`/Engine/EditorBlueprintResources/StandardMacros.IsValid` (`self.FirstCharaRef`)
    (:`Is Valid`
      (`SceneComponent.K2_SetWorldRotation` _camera (`KismetMathLibrary.FindLookAtRotation` (`SceneComponent.K2_GetComponentLocation` _camera) (`SceneComponent.K2_GetComponentLocation` (`/Game/Blueprint/Character/BP_FirstChara.SniperCompTarget` (`self.FirstCharaRef`)))) false false))))

(fn `UserConstructionScript`)