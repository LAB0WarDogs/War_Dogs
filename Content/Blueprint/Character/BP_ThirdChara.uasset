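; Third playable character, a child of a master character class, with smoke, trap and distance-hack skills.
; Overrides of the parent's activate, use and cancel functions call the parent, then route to the matching skill object by active-skill flags.
; A timeline lerps spring arm length to zoom the camera out and back.
; It also binds inventory battery use on BeginPlay and forwards damage to the parent's handling.
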(event `Zoom`
  ;[0 0 1] Timeline Zoom Dezoom
  (`TimelineComponent.SetPlayRate` (`self.ZoomDezoomTL`) (/ 1.0 (`self.ZoomDezoomTimeSniperSkill`)))
  (bind (_direction _zoom_dezoom) (`Timeline|ZoomDezoomTL` :!label _label)
    (:`Update`
      (set `SpringArmComponent.TargetArmLength` (`KismetMathLibrary.Lerp` 1200.0 1600.0 _zoom_dezoom) (`self.SpringArm`)))))

(event `self.ReceiveBeginPlay`
  ;[0 0 1] Comment
  (`parent.ReceiveBeginPlay`)
  (bind _ascharacter_master (`/Game/Blueprint/FL_Main.Get Player Character Master`))
  (add `self.UseBatteryFromInventory` _ascharacter_master (delegate `UsingBattery-ThirdChara`)))

(event `UsingBattery-ThirdChara`
  ;[0 0 1] Comment
  (`self.UseBattery`))

(event `Dezoom`
  ;[0 0 1] Timeline Zoom Dezoom
  (goto _label :!via `ReverseFromEnd`))

(event `/Game/Blueprint/Interface/BPI_Damageable.TakeDamage`
  (params (Damage :type "Float (double-precision)"))
  ;[0 0 1] Take Damage
  (`self.TakeDamageFromEnnemyOrFriend` Damage))

(fn `ActivateFirstSkill`
  (`parent.ActivateFirstSkill`)
  (`/Game/Blueprint/SkiilsActorComponent/BP_SmokeSkills.ActivateFirstSkill` (`self.BP_SmokeSkills`))
  (`KismetSystemLibrary.PrintString` "Fitstskill"))

(fn `ActivateSecondSkill`
  (`parent.ActivateSecondSkill`)
  (`/Game/Blueprint/SkiilsActorComponent/BP_TrapSkills.ActivateThirdSkill` (`self.BP_Trap`))
  (`KismetSystemLibrary.PrintString` "ThirdSkill"))

(fn `ActivateThirdSkill`
  (`parent.ActivateThirdSkill`)
  (`/Game/Blueprint/SkiilsActorComponent/BP_HackDistanceSkill.ActivateThirdSkill` (`self.BP_HackDistanceSkill`)))

(fn `CancelSkill`
  (params (`FirstSkillActive?` :type Boolean) (`SecondSkillActive?` :type Boolean) (`ThirdSkillActive?` :type Boolean))
  (`parent.CancelSkill` `FirstSkillActive?` `SecondSkillActive?` `ThirdSkillActive?`)
  (if (`local.FirstSkillActive?`)
    (`/Game/Blueprint/SkiilsActorComponent/BP_SmokeSkills.Cancelation` (`self.BP_SmokeSkills`))
    (elif (`local.SecondSkillActive?`)
      (`/Game/Blueprint/SkiilsActorComponent/BP_TrapSkills.CancelTrapSkill` (`self.BP_Trap`))
      (elif (`self.ThirdSkillActivated?`)
        (`/Game/Blueprint/SkiilsActorComponent/BP_HackDistanceSkill.Cancelation` (`self.BP_HackDistanceSkill`))))))

(fn `GetHealth`
  (params (DamageTaken :type "Float (double-precision)"))
  (`parent.GetHealth` DamageTaken))

(fn `TakeDamageFromEnnemyOrFriend`
  (params (DamageTaken :type "Float (double-precision)"))
  (`parent.TakeDamageFromEnnemyOrFriend` DamageTaken))

(fn `UseFirstSkill`
  (params (`FirstSkillActive?` :type Boolean) (`SecondSkillActive?` :type Boolean) (`ThirdSkillActive?` :type Boolean))
  (`parent.UseFirstSkill` `FirstSkillActive?` `SecondSkillActive?` `ThirdSkillActive?`)
  (if (`local.FirstSkillActive?`)
    (`/Game/Blueprint/SkiilsActorComponent/BP_SmokeSkills.UsingFirstSkill` (`self.BP_SmokeSkills`))
    (elif (`self.SecondarySkillActivated?`)
      (`/Game/Blueprint/SkiilsActorComponent/BP_TrapSkills.UsingSecondSkill` (`self.BP_Trap`))
      (elif (`local.ThirdSkillActive?`)
        (`/Game/Blueprint/SkiilsActorComponent/BP_HackDistanceSkill.UseHackDistanceSkill` (`self.BP_HackDistanceSkill`))))))

(fn `UserConstructionScript`
  (`parent.UserConstructionScript`))