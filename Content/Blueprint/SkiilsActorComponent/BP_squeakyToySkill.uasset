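; Skill component that lets the second character (BP_SecondChara) use a squeaky toy as its second skill.
; Activation checks cooldown and skill state, sets the character's usage flags and shows the toy position component, then after a short delay spawns BP_SkeaquyToy there.
; It then clears the flags, hides that component, notifies the player's CharacterMaster to start the cooldown and re-enables itself via a timed delay.
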(event `self.ReceiveBeginPlay`
  (bind _returnvalue (`GameplayStatics.GetActorOfClass` "/Game/Blueprint/Character/BP_SecondChara.BP_SecondChara_C"))
  (set `self.SecondCharaRef` _returnvalue)
  (bind _ascharacter_master (`/Game/Blueprint/FL_Main.Get Player Character Master`))
  (set `self.As Character Master` _ascharacter_master))

(event `ActivateSecondSkill`
  (if (and (not (`/Game/Blueprint/Character/CharacterMaster.IsUsingSkill` (`self.SecondCharaRef`))) (`self.CooldownOver?`))
    (set `/Game/Blueprint/Character/CharacterMaster.IsUsingSkill` true (`self.SecondCharaRef`))
    (set `/Game/Blueprint/Character/BP_SecondChara.IsUsingSqueakyToy` true (`self.SecondCharaRef`))
    (`SceneComponent.SetVisibility` (`/Game/Blueprint/Character/BP_SecondChara.SqueakyToyPos` (`self.SecondCharaRef`)) true false)
    (`KismetSystemLibrary.Delay` 1.0)
    (`self.UseSecondSkill`)))

(event `UseSecondSkill`
  (bind _cooldownbeforeactifagain (`self.CooldownBeforeActifAgain`))
  (bind _returnvalue_location (`KismetMathLibrary.BreakTransform` (`SceneComponent.K2_GetComponentToWorld` (`/Game/Blueprint/Character/BP_SecondChara.SqueakyToyPos` (`self.SecondCharaRef`)))))
  (if (`self.CooldownOver?`)
    (`|SpawnActorFromClass` "/Game/Blueprint/Actors/squeakyToy/BP_SkeaquyToy.BP_SkeaquyToy_C" (`KismetMathLibrary.MakeTransform` _returnvalue_location) "Undefined" "OverrideRootScale" null null)
    (set `self.CooldownOver?` false)
    (set `/Game/Blueprint/Character/CharacterMaster.IsUsingSkill` false (`self.SecondCharaRef`))
    (`KismetSystemLibrary.Delay` 0.5)
    (set `/Game/Blueprint/Character/BP_SecondChara.IsUsingSqueakyToy` false (`self.SecondCharaRef`))
    (`SceneComponent.SetVisibility` (`/Game/Blueprint/Character/BP_SecondChara.SqueakyToyPos` (`self.SecondCharaRef`)) false false)
    (`/Game/Blueprint/Character/CharacterMaster.StartCooldown` (`self.As Character Master`) _cooldownbeforeactifagain)
    (`KismetSystemLibrary.Delay` _cooldownbeforeactifagain)
    (set `self.CooldownOver?` true)))