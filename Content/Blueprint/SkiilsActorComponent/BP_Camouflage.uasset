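; BP_Camouflage is the player's third skill, a timed camouflage that spends a battery and starts a cooldown.
; It slows global time, boosts the player's own time dilation, calls the character's camo state and spawns a hidden BP_HidingBush that a looping timer keeps on the player.
; Halfway through the duration the mesh flickers as a warning, then time, visibility and skill flags are restored and the bush is destroyed.
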(event `self.ReceiveBeginPlay`
  (`|ExecutionSequence`
    (:`then_0`
      (bind _asbp_first_chara (cast `/Game/Blueprint/Character/BP_FirstChara` (`GameplayStatics.GetPlayerCharacter` 0)))
      (set `self.As BP First Chara` _asbp_first_chara))
    (:`then_1`
      (bind _ascharacter_master (`/Game/Blueprint/FL_Main.Get Player Character Master`))
      (set `self.As Character Master` _ascharacter_master))))

(event `setHidingPos`
  (bind _returnvalue_location (`KismetMathLibrary.BreakTransform` (`Actor.GetTransform` (`self.As BP First Chara`))))
  ;[1 1 1] A modifier plus tard pour rendre plus propre
  (`Actor.K2_SetActorLocation` (stale `ActivateThirdSkill` _returnvalue) _returnvalue_location false false))

(event `ActivateThirdSkill`
  (bind _as_bp_first_chara (`self.As BP First Chara`))
  (bind _returnvalue_location (`KismetMathLibrary.BreakTransform` (`Actor.GetTransform` _as_bp_first_chara)))
  (if (not (`/Game/Blueprint/Character/CharacterMaster.IsUsingSkill` (`self.As BP First Chara`)))
    (set `self.CamoIsActive?` true)
    (set `/Game/Blueprint/Character/CharacterMaster.IsUsingSkill` true (`self.As BP First Chara`))
    (set `/Game/Blueprint/Character/CharacterMaster.CanMoveWithUsingSkill` true _as_bp_first_chara)
    (`self.UseStealthSkill`)
    ;[1 1 1] A modifier plus tard pour rendre plus propre
    (bind _returnvalue (`|SpawnActorFromClass` "/Game/Blueprint/WorldMechanics/HidingBush/BP_HidingBush.BP_HidingBush_C" (`KismetMathLibrary.MakeTransform` _returnvalue_location (struct) (2.0 2.0 2.0)) "AdjustIfPossibleButAlwaysSpawn" "OverrideRootScale" null null))
    (bind _returnvalue_2 (`KismetSystemLibrary.K2_SetTimerDelegate` (delegate `setHidingPos`) 0.01 true))
    (`Actor.SetActorHiddenInGame` _returnvalue true)))

(event `Cancelation`
  (set `/Game/Blueprint/Character/CharacterMaster.IsUsingSkill` false (`self.As BP First Chara`) :!label _label)
  (set `/Game/Blueprint/Character/CharacterMaster.CanMoveWithUsingSkill` false (`self.As BP First Chara`)))

(event `UseStealthSkill`
  (bind _cooldownforstealthmode (`self.CoolDownForStealthMode`))
  (bind _returnvalue (- _cooldownforstealthmode (* (`self.CoolDownForStealthMode`) 0.5)))
  (if (`self.CamoIsActive?`)
    (`/Game/Blueprint/Character/CharacterMaster.UseBatteryFromInventory` (`self.As Character Master`))
    (set `self.CamoIsActive?` false)
    (`GameplayStatics.SetGlobalTimeDilation` 0.5)
    (bind _asbp_first_chara (cast `/Game/Blueprint/Character/BP_FirstChara` (`GameplayStatics.GetPlayerCharacter` 0)))
    (set `Actor.CustomTimeDilation` 1.5 _asbp_first_chara)
    (`/Game/Blueprint/Character/BP_FirstChara.UsingCamo` _asbp_first_chara)
    (`/Game/Blueprint/Character/CharacterMaster.StartCooldown` (`self.As Character Master`) _cooldownforstealthmode)
    (`KismetSystemLibrary.Delay` _returnvalue)
    (`self.StartFlickering`)
    (`KismetSystemLibrary.Delay` (- (`self.CoolDownForStealthMode`) _returnvalue))
    (`/Game/Blueprint/Character/BP_FirstChara.StopUsingCamo` _asbp_first_chara)
    (goto _label)))

(event `StartFlickering`
  (bind _returnvalue (`KismetSystemLibrary.K2_SetTimerDelegate` (delegate `Flicker`) 0.1 true))
  (`KismetSystemLibrary.Delay` (- (`self.CoolDownForStealthMode`) (- (`self.CoolDownForStealthMode`) (* (`self.CoolDownForStealthMode`) 0.5))))
  (`KismetSystemLibrary.K2_ClearAndInvalidateTimerHandle` _returnvalue)
  (`SceneComponent.SetVisibility` (`Character.Mesh` (`self.As BP First Chara`)) true false)
  (`GameplayStatics.SetGlobalTimeDilation` 1.0)
  (set `Actor.CustomTimeDilation` 1.0 (stale `UseStealthSkill` _asbp_first_chara))
  ;[1 1 1] A modifier plus tard pour rendre plus propre
  (`Actor.K2_DestroyActor` (stale `ActivateThirdSkill` _returnvalue))
  (`KismetSystemLibrary.K2_ClearAndInvalidateTimerHandle` (stale `ActivateThirdSkill` _returnvalue_2)))

(event `Flicker`
  (`SceneComponent.ToggleVisibility` (`Character.Mesh` (`self.As BP First Chara`)) false))