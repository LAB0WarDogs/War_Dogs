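; Player skill component for an aimed sniper shot.
; Aiming halves global time, zooms, shows the noise radius, and turns the character toward an offset target tracking the mouse/joystick cursor.
; Firing blends to BP_ShootCamera, freezes AI through custom time dilation, box-traces to the target, damages BPI_Damageable hits and reports AI noise.
; Firing and cancelling share cleanup restoring time, camera and state, with the long cooldown skipped on cancel.
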(event `self.ReceiveTick`
  (params (DeltaSeconds :type "Float (single-precision)"))
  (bind (_sizex _sizey) (`PlayerController.GetViewportSize` (`GameplayStatics.GetPlayerController` 0)))
  (bind _asmy_player_controller (`/Game/Blueprint/FL_Main.GetPlayerController`))
  (bind (_locationx _locationy) (`PlayerController.GetMousePosition` _asmy_player_controller))
  (`PlayerController.SetMouseLocation` (`GameplayStatics.GetPlayerController` 0) (`KismetMathLibrary.Clamp` (`KismetMathLibrary.FTrunc` (+ _locationx (* (`/Game/Blueprint/Character/MyPlayerController.JoystickX` _asmy_player_controller) 20.0))) 0 _sizex) (`KismetMathLibrary.Clamp` (`KismetMathLibrary.FTrunc` (+ _locationy (* (`/Game/Blueprint/Character/MyPlayerController.JoystickY` _asmy_player_controller) 20.0))) 0 _sizey))
  (`/Game/Blueprint/Character/BP_FirstChara.CursorMovement` (`self.As BP First Chara`))
  (`KismetSystemLibrary.MoveComponentTo` (`self.Sniper Comp Target`) (+ (`.ImpactPoint` (`GameplayStatics.BreakHitResult` (`PlayerController.GetHitResultUnderCursorByChannel` (`GameplayStatics.GetPlayerController` 0) "TraceTypeQuery1" true))) (+ (`KismetMathLibrary.VLerp` (-25.0 0.0 0.0) (25.0 0.0 0.0) (`self.Alpha`)) (`KismetMathLibrary.VLerp` (0.0 -25.0 0.0) (0.0 25.0 0.0) (`self.Alpha_0`)))) (struct) false false (* (`self.OverTimeSpeed`) (`GameplayStatics.GetWorldDeltaSeconds`))))

(event `self.ReceiveBeginPlay`
  (`|ExecutionSequence`
    (:`then_0`
      (bind _asbp_first_chara (cast `/Game/Blueprint/Character/BP_FirstChara` (`GameplayStatics.GetPlayerCharacter` 0)))
      (set `self.As BP First Chara` _asbp_first_chara)
      (set `self.Sniper Comp Target` (`/Game/Blueprint/Character/BP_FirstChara.SniperCompTarget` _asbp_first_chara))
      (set `self.Spring Arm` (`/Game/Blueprint/Character/CharacterMaster.SpringArm` _asbp_first_chara)))
    (:`then_1`
      (bind _ascharacter_master (`/Game/Blueprint/FL_Main.Get Player Character Master`))
      (set `self.As Character Master` _ascharacter_master))))

(event `ActivateSniperSkill`
  (if (and (not (`/Game/Blueprint/Character/CharacterMaster.IsUsingSkill` (`self.As BP First Chara`))) (`self.CoolDownIsOver?`))
    (`self.SetComponentTickEnabled` true)
    (set `/Game/Blueprint/Character/CharacterMaster.IsUsingSkill` true (`self.As BP First Chara`))
    (`self.AimSniperSkill`)))

(event `AimSniperSkill`
  (bind (_sizex _sizey) (`PlayerController.GetViewportSize` (`GameplayStatics.GetPlayerController` 0)))
  (bind _noisearea (`/Game/Blueprint/Character/CharacterMaster.NoiseArea` (`self.As BP First Chara`)))
  (set `self.CoolDownIsOver?` false)
  (set `self.FacePlayer?` true)
  (`self.AlwaysFacePlayer`)
  (`SceneComponent.SetVisibility` (`self.Sniper Comp Target`) true true)
  (`SceneComponent.K2_DetachFromComponent` (`self.Sniper Comp Target`) "KeepWorld" "KeepWorld" "KeepWorld" true)
  (`/Game/Blueprint/Character/BP_FirstChara.Zoom` (`self.As BP First Chara`))
  (`PlayerController.SetMouseLocation` (`GameplayStatics.GetPlayerController` 0) (/ _sizex 2) (/ _sizey 2))
  (`GameplayStatics.SetGlobalTimeDilation` 0.5)
  (`SceneComponent.SetWorldScale3D` _noisearea (30.0 30.0 0.1))
  (`SceneComponent.SetVisibility` _noisearea true true))

(event `Cancelation`
  (bind (_sizex _sizey) (`PlayerController.GetViewportSize` (`GameplayStatics.GetPlayerController` 0)))
  (bind _noisearea (`/Game/Blueprint/Character/CharacterMaster.NoiseArea` (`self.As BP First Chara`)))
  (if (`self.UseSkillHasBeenPressed?`)
    (set `self.IsCanceled` true)
    (`SceneComponent.SetVisibility` (`self.Sniper Comp Target`) false true :!label _label)
    (`GameplayStatics.SetGlobalTimeDilation` 1.0)
    (`|ExecutionSequence`
      (:`then_0`
        (bind _outactors (`GameplayStatics.GetAllActorsOfClass` "/Game/Blueprint/AI/AI_Puces/AiCharacter/BP_AI_Master.BP_AI_Master_C"))
        (for _array_element _outactors
          (`/Engine/EditorBlueprintResources/StandardMacros.IsValid` _array_element
            (:`Is Valid`
              (set `Actor.CustomTimeDilation` 1.0 _array_element))
            (:`Is Not Valid`
              (set `self.FacePlayer?` false :!label _label_2)
              (`/Game/Blueprint/Character/BP_FirstChara.Dezoom` (`self.As BP First Chara`))
              (if (not (`self.IsCanceled`))
                (`KismetSystemLibrary.Delay` (`self.CooldownDuration`))
                (else
                  (set `self.IsCanceled` false)))
              (`PlayerController.SetMouseLocation` (`GameplayStatics.GetPlayerController` 0) (/ _sizex 2) (/ _sizey 2))
              (bind _ascharacter_master (`/Game/Blueprint/FL_Main.Get Player Character Master`))
              (set `/Game/Blueprint/Character/CharacterMaster.PrimarySkillActivated?` false _ascharacter_master)
              (set `/Game/Blueprint/Character/CharacterMaster.IsUsingSkill` false (`self.As BP First Chara`))
              (`PlayerController.SetViewTargetWithBlend` (`GameplayStatics.GetPlayerController` 0) (`self.As BP First Chara`) 1.0 "VTBlend_Linear" 0.0 false)
              (`/Game/Blueprint/Character/CharacterMaster.StartCooldown` (`self.As Character Master`) 1.0)
              (`KismetSystemLibrary.Delay` 1.0)
              (`self.SetComponentTickEnabled` false)
              (set `self.UseSkillHasBeenPressed?` true)
              (set `self.CoolDownIsOver?` true))))
        (goto _label_2))
      (:`then_1`
        (`KismetSystemLibrary.Delay` 1.0)
        (`SceneComponent.SetWorldScale3D` _noisearea (10.0 10.0 0.1))
        (`SceneComponent.SetVisibility` _noisearea false true)))))

(event `UseSniperSkill`
  (bind _as_bp_first_chara (`self.As BP First Chara`))
  (bind _as_bp_first_chara_2 (`self.As BP First Chara`))
  (bind _returnvalue (`SceneComponent.K2_GetComponentLocation` (`Character.CapsuleComponent` _as_bp_first_chara_2)))
  (bind _returnvalue_2 (`SceneComponent.K2_GetComponentLocation` (`Character.CapsuleComponent` _as_bp_first_chara)))
  (if (`self.UseSkillHasBeenPressed?`)
    (set `self.UseSkillHasBeenPressed?` false)
    ;[1 1 1] Comment
    (bind _returnvalue_3 (`GameplayStatics.GetActorOfClass` "/Game/Blueprint/Character/BP_ShootCamera.BP_ShootCamera_C"))
    (`PlayerController.SetViewTargetWithBlend` (`GameplayStatics.GetPlayerController` 0) _returnvalue_3 0.2 "VTBlend_Linear" 0.0 false)
    (bind _outhit (`KismetSystemLibrary.BoxTraceSingle` :`Start` (`SceneComponent.K2_GetComponentLocation` (`/Game/Blueprint/Character/BP_FirstChara.SniperSkillStartPoint` (`self.As BP First Chara`))) :`End` (`SceneComponent.K2_GetComponentLocation` (`self.Sniper Comp Target`)) :`HalfSize` (10.0 10.0 10.0) :`TraceChannel` "TraceTypeQuery1" :`DrawDebugType` "ForDuration"))
    (bind _outactors (`GameplayStatics.GetAllActorsOfClass` "/Game/Blueprint/AI/AI_Puces/AiCharacter/BP_AI_Master.BP_AI_Master_C"))
    (for _array_element _outactors
      (set `Actor.CustomTimeDilation` 0.0 _array_element)
      (`self.SetComponentTickEnabled` false)
      (bind (_bblockinghit _binitialoverlap _time _distance _location _impactpoint _normal _impactnormal _physmat _hitactor _hitcomponent) (`GameplayStatics.BreakHitResult` _outhit))
      (`KismetSystemLibrary.PrintString` (`KismetSystemLibrary.GetDisplayName` _hitactor))
      (if (or (`KismetSystemLibrary.DoesImplementInterface` _hitactor "/Game/Blueprint/Interface/BPI_Damageable.BPI_Damageable_C") (`KismetSystemLibrary.DoesImplementInterface` _hitcomponent "/Game/Blueprint/Interface/BPI_Damageable.BPI_Damageable_C"))
        ;[1 1 1] Comment
        (`KismetSystemLibrary.Delay` 0.3)
        (`GameplayStatics.PlaySoundAtLocation` "/Engine/VREditor/Sounds/UI/Foliage_Placed.Foliage_Placed" _returnvalue (struct) 1.0 1.0 0.0 null null null null)
        (`AISense_Hearing.ReportNoiseEvent` _returnvalue 1.0 _as_bp_first_chara_2 1500.0)
        (message `/Game/Blueprint/Interface/BPI_Damageable.TakeDamage` _hitactor 110.0)
        (goto _label)
        (else
          (`KismetSystemLibrary.Delay` 0.25)
          (`GameplayStatics.PlaySoundAtLocation` "/Engine/VREditor/Sounds/UI/Foliage_Placed.Foliage_Placed" _returnvalue_2 (struct) 1.0 1.0 0.0 null null null null)
          (`AISense_Hearing.ReportNoiseEvent` _returnvalue_2 1.0 _as_bp_first_chara 1500.0)
          (goto _label))))))

(event `AlwaysFacePlayer`
  (bind (_returnvalue_roll _returnvalue_pitch _returnvalue_yaw) (`KismetMathLibrary.BreakRotator` (`KismetMathLibrary.RInterpTo` (`Actor.K2_GetActorRotation` (`self.As BP First Chara`)) (`KismetMathLibrary.FindLookAtRotation` (`Actor.K2_GetActorLocation` (`self.As BP First Chara`)) (`SceneComponent.RelativeLocation` (`self.Sniper Comp Target`))) (`GameplayStatics.GetWorldDeltaSeconds`) 20.0)))
  (if (`self.FacePlayer?`)
    (`Actor.K2_SetActorRelativeRotation` (`self.As BP First Chara`) (`KismetMathLibrary.MakeRotator` 0.0 0.0 _returnvalue_yaw) false false)
    (`KismetSystemLibrary.Delay` 0.001)
    (`self.AlwaysFacePlayer`)))