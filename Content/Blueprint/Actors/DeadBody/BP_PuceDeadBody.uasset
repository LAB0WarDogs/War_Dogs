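; BP_PuceDeadBody is a dead-body actor for a Puce that AI can detect by sight until it is checked.
; Initialization stores the owner and supplied location, then after a search-zone delay replaces that location with the body's current one.
; CheckDeadBody flags the body as checked, makes its sphere ignore a custom trace channel and unregisters its perception stimulus from sight.
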(event `InitializationDeadBody`
  (params (Vector3 :type "Vector Structure") (Actor :type "Actor Object Reference"))
  (set `self.PuceOwner` Actor)
  (set `self.ActorLocation` Vector3)
  (`KismetSystemLibrary.Delay` (`self.DelayChercheZone`))
  (set `self.ActorLocation` (`self.K2_GetActorLocation` self)))

(event `CheckDeadBody`
  (set `self.Check` true)
  (`PrimitiveComponent.SetCollisionResponseToChannel` (`self.Sphere`) "ECC_GameTraceChannel4" "ECR_Ignore")
  (`AIPerceptionStimuliSourceComponent.UnregisterFromSense` (`self.AIPerceptionStimuliSource`) "/Script/AIModule.AISense_Sight"))

(fn `UserConstructionScript`)