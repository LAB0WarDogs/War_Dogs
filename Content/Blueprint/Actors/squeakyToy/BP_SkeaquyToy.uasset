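; BP_SkeaquyToy is a short-lived squeaky toy actor that makes noise as soon as it begins play.
; It finds BP_SecondChara, shows that character's NoiseArea and widens it in X and Y.
; It plays the squeak at its location and reports a range-limited noise event there, with itself as instigator.
; After a brief delay it restores the NoiseArea scale, leaving it visible, and destroys itself.
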(event `self.ReceiveBeginPlay`
  (bind _returnvalue (`self.K2_GetActorLocation`))
  (`|ExecutionSequence`
    (:`then_0`
      (bind _returnvalue_2 (`GameplayStatics.GetActorOfClass` "/Game/Blueprint/Character/BP_SecondChara.BP_SecondChara_C"))
      (bind _noisearea (`/Game/Blueprint/Character/CharacterMaster.NoiseArea` _returnvalue_2))
      (set `self.Noise Area` _noisearea)
      (set `self.OriginalWorldScale` (`SceneComponent.K2_GetComponentScale` _noisearea))
      (`SceneComponent.SetVisibility` _noisearea true false)
      (bind (_returnvalue_x _returnvalue_y _returnvalue_z) (`KismetMathLibrary.BreakVector` (`SceneComponent.K2_GetComponentScale` _noisearea)))
      (`SceneComponent.SetWorldScale3D` _noisearea (`KismetMathLibrary.MakeVector` (+ _returnvalue_x 10.0) (+ _returnvalue_y 10.0) _returnvalue_z)))
    (:`then_1`
      (`GameplayStatics.PlaySoundAtLocation` "/Game/Sound/SqueakyToy/SqueatyToy_Cue.SqueatyToy_Cue" _returnvalue (struct) 1.0 1.0 0.0 null null null null)
      (`AISense_Hearing.ReportNoiseEvent` _returnvalue 1.0 self 1000.0)
      (`KismetSystemLibrary.Delay` 1.0)
      (`SceneComponent.SetWorldScale3D` (`self.Noise Area`) (`self.OriginalWorldScale`))
      (`self.K2_DestroyActor`))))

(fn `UserConstructionScript`)