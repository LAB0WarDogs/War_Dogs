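; BP_Smoke is a smoke grenade actor that creates a temporary smoke effect with a collidable StaticMesh.
; On BeginPlay it disables mesh collision, then after a short fuse plays a sound, hides the Sphere and its children, and enables mesh collision.
; It spawns the NS_SmokeGrenade Niagara system at the mesh, then destroys the effect and itself after LifeTime.
; A node that would make the StaticMesh visible is disconnected.
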(event `self.ReceiveBeginPlay`
  (`PrimitiveComponent.SetCollisionEnabled` (`self.StaticMesh`) "NoCollision")
  (`KismetSystemLibrary.Delay` 2.5)
  (`GameplayStatics.PlaySoundAtLocation` "/Engine/VREditor/Sounds/UI/Teleport_Committed.Teleport_Committed" (`self.K2_GetActorLocation`) (struct) 1.0 1.0 0.0 null null null null)
  (`SceneComponent.SetVisibility` (`self.Sphere`) false true)
  (`PrimitiveComponent.SetCollisionEnabled` (`self.StaticMesh`) "QueryAndPhysics")
  (bind _returnvalue (`NiagaraFunctionLibrary.SpawnSystemAtLocation` "/Game/VFX/Smoke/NS_SmokeGrenade.NS_SmokeGrenade" (`SceneComponent.K2_GetComponentLocation` (`self.StaticMesh`))))
  (`KismetSystemLibrary.Delay` (`self.LifeTime`))
  (`ActorComponent.K2_DestroyComponent` _returnvalue)
  (`self.K2_DestroyActor`))

(fn `UserConstructionScript`)