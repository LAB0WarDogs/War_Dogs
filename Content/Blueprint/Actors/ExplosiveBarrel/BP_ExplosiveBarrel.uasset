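; Explosive barrel that BP_SecondChara can pick up, carry on a mesh socket and set down via a line trace when space allows.
; An overlap box shows the interaction widget, and a looping timer handles damage-area display on cursor hover.
; At zero health it plays effects, reports noise and sphere-checks for BPI_Damageable actors.
; Each such actor found takes damage and triggers a BP_Bomb field explosion and delayed barrel destruction.
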(event `self.ReceiveBeginPlay`
  (`KismetSystemLibrary.Delay` 0.1)
  (bind _returnvalue (`GameplayStatics.GetActorOfClass` "/Game/Blueprint/Character/BP_SecondChara.BP_SecondChara_C"))
  (set `self.SecondCharaRef` _returnvalue)
  (bind _returnvalue_2 (`KismetSystemLibrary.K2_SetTimerDelegate` (`|CreateDelegate` :!event `SetDamageAreaVisibility`) 0.1 true))
  (set `self.DamageAreaVisibilityTimer` _returnvalue_2))

(event `/Game/Blueprint/Interface/BPI_Damageable.TakeDamage`
  (params (Damage :type "Float (double-precision)"))
  (bind _returnvalue (`self.K2_GetActorLocation`))
  (bind _returnvalue_2 (`SceneComponent.K2_GetComponentLocation` (`self.Cylinder`)))
  (set `self.Health` (- (`self.Health`) Damage))
  (if (<= (`self.Health`) 0.0)
    (`KismetSystemLibrary.K2_ClearAndInvalidateTimerHandle` (`self.DamageAreaVisibilityTimer`))
    (`NiagaraFunctionLibrary.SpawnSystemAtLocation` "/Game/VFX/Explosion/NS_Explosion.NS_Explosion" (`self.K2_GetActorLocation`) (struct) (3.0 3.0 3.0))
    (`GameplayStatics.PlaySoundAtLocation` "/Engine/EditorSounds/GamePreview/StartPlayInEditor.StartPlayInEditor" _returnvalue_2 (struct) 1.0 1.0 0.0 null null null null)
    (`AISense_Hearing.ReportNoiseEvent` _returnvalue_2 1.0 self 2000.0)
    (`SceneComponent.SetVisibility` (`self.Cylinder`) false false)
    (`KismetSystemLibrary.Delay` 0.1)
    (bind _outactors (`KismetSystemLibrary.SphereOverlapActors` _returnvalue (`self.Sphere Radius`) (`self.Object Types`) null (`|MakeArray` self :!type "Actor Object Reference")))
    (`KismetSystemLibrary.DrawDebugSphere` _returnvalue (`self.Sphere Radius`) 12 (struct :`R` 1.0 :`G` 1.0 :`B` 1.0 :`A` 1.0) 1.0)
    (for _array_element _outactors
      (`/Engine/EditorBlueprintResources/StandardMacros.IsValid` _array_element
        (:`Is Valid`
          (if (`KismetSystemLibrary.DoesImplementInterface` _array_element "/Game/Blueprint/Interface/BPI_Damageable.BPI_Damageable_C")
            (message `/Game/Blueprint/Interface/BPI_Damageable.TakeDamage` _array_element 110.0)
            (message `/Game/Blueprint/Interface/BPI_Damageable.EnvironmentTakingDamage` _array_element)
            (bind _returnvalue_3 (`|SpawnActorFromClass` "/Game/Blueprint/WorldMechanics/DestructibleWalls/BP_Bomb.BP_Bomb_C" (`KismetMathLibrary.MakeTransform` (`SceneComponent.K2_GetComponentLocation` (`self.Cylinder`))) "Undefined" "OverrideRootScale" null null))
            (`/Game/Blueprint/WorldMechanics/DestructibleWalls/BP_Bomb.Explode` _returnvalue_3 (`self.Field Magnitude`))
            (`KismetSystemLibrary.Delay` 0.1)
            (`self.K2_DestroyActor`)))))))

(event `/Game/Blueprint/Interface/BPI_InteractInterface.Interact`
  (bind _secondchararef (`self.SecondCharaRef`))
  (bind _secondchararef_2 (`self.SecondCharaRef`))
  (if (and (not (`self.IsAttached`)) (`self.CanInteract`))
    (`CharacterMovementComponent.DisableMovement` (`Character.CharacterMovement` (`self.SecondCharaRef`)))
    (`PrimitiveComponent.SetCollisionEnabled` (`self.Cylinder`) "NoCollision")
    (set `/Game/Blueprint/Character/CharacterMaster.IsUsingSkill` true _secondchararef_2)
    (set `/Game/Blueprint/Character/CharacterMaster.CanMoveWithUsingSkill` true _secondchararef_2)
    (`/Engine/EditorBlueprintResources/StandardMacros.IsValid` _secondchararef
      (:`Is Valid`
        (`self.K2_AttachToComponent` (`Character.Mesh` _secondchararef) "BarilsSocket" "SnapToTarget" "SnapToTarget" "KeepWorld")
        (set `/Game/Blueprint/Character/BP_SecondChara.IsCarryingBarrel` true (`self.SecondCharaRef`))
        (`SceneComponent.SetHiddenInGame` (`self.Widget`) true false)
        (`KismetSystemLibrary.Delay` 1.2)
        (set `self.IsAttached` true)
        (`CharacterMovementComponent.SetMovementMode` (`Character.CharacterMovement` (`self.SecondCharaRef`)) "MOVE_Walking" 0)
        (`/Game/Blueprint/Character/CharacterMaster.CheckIfEnoughSpace` (`self.SecondCharaRef`) (`self.Max Distance for Detection`))
        (`PrimitiveComponent.SetCollisionResponseToChannel` (`self.Box`) "ECC_GameTraceChannel5" "ECR_Ignore")
        (`PrimitiveComponent.SetCollisionResponseToChannel` (`self.Cylinder`) "ECC_GameTraceChannel5" "ECR_Ignore")))))

(event `/Game/Blueprint/Interface/BPI_InteractInterface.StopInteracting`
  (bind _secondchararef (`self.SecondCharaRef`))
  (`self.CheckIfCanBePlacedDown`)
  (if (and (`self.IsAttached`) (not (`/Game/Blueprint/Character/CharacterMaster.CannotBePlaced` (`self.SecondCharaRef`))))
    (`PrimitiveComponent.SetCollisionEnabled` (`self.Cylinder`) "QueryAndPhysics")
    (`PrimitiveComponent.SetCollisionResponseToChannel` (`self.Box`) "ECC_GameTraceChannel5" "ECR_Block")
    (`PrimitiveComponent.SetCollisionResponseToChannel` (`self.Cylinder`) "ECC_GameTraceChannel5" "ECR_Block")
    (bind _outhit (`KismetSystemLibrary.LineTraceSingle` :`Start` (`self.K2_GetActorLocation` (`self.SecondCharaRef`)) :`End` (+ (- (`self.K2_GetActorLocation` (`self.SecondCharaRef`)) (0.0 0.0 500.0)) (* (`self.GetActorForwardVector` (`self.SecondCharaRef`)) 1000.0)) :`TraceChannel` "TraceTypeQuery1" :`DrawDebugType` "ForDuration"))
    (`self.K2_DetachFromActor` self "KeepWorld" "KeepWorld" "KeepWorld")
    (bind (_bblockinghit _binitialoverlap _time _distance _location _impactpoint) (`GameplayStatics.BreakHitResult` _outhit))
    (`self.K2_SetActorTransform` self (`KismetMathLibrary.MakeTransform` (`KismetMathLibrary.MakeVector` (.x _impactpoint) (.y _impactpoint) (+ (.z _impactpoint) 50.0))) false false)
    (`SceneComponent.SetHiddenInGame` (`self.Widget`) false false)
    (set `self.IsAttached` false)
    (`/Game/Blueprint/Character/CharacterMaster.ResetTimerEnoughSpace` (`self.SecondCharaRef`))
    (set `/Game/Blueprint/Character/CharacterMaster.IsUsingSkill` false _secondchararef)
    (set `/Game/Blueprint/Character/CharacterMaster.CanMoveWithUsingSkill` true _secondchararef)
    (set `/Game/Blueprint/Character/BP_SecondChara.IsCarryingBarrel` false (`self.SecondCharaRef`))))

(event `self.Box.OnComponentBeginOverlap`
  (params (OverlappedComponent :type "PrimitiveComponent Object Reference") (OtherActor :type "Actor Object Reference") (OtherComp :type "PrimitiveComponent Object Reference") (OtherBodyIndex :type Integer) (bFromSweep :type Boolean) (SweepResult :type "HitResult Structure (by ref)"))
  (cast `/Game/Blueprint/Character/BP_SecondChara` OtherActor)
  (`SceneComponent.SetVisibility` (`self.Widget`) true false)
  (set `self.CanInteract` true))

(event `CheckIfCanBePlacedDown`
  (if (`/Game/Blueprint/Character/CharacterMaster.CannotBePlaced` (`self.SecondCharaRef`))
    (`GameplayStatics.PlaySoundAtLocation` "/Game/Sound/SqueakyToy/SqueatyToy.SqueatyToy" (`self.K2_GetActorLocation`) (struct) 1.0 1.0 0.0 null null null null)))

(event `self.Box.OnComponentEndOverlap`
  (params (OverlappedComponent :type "PrimitiveComponent Object Reference") (OtherActor :type "Actor Object Reference") (OtherComp :type "PrimitiveComponent Object Reference") (OtherBodyIndex :type Integer))
  (cast `/Game/Blueprint/Character/BP_SecondChara` OtherActor)
  (`SceneComponent.SetVisibility` (`self.Widget`) false false)
  (set `self.CanInteract` false))

(event `SetDamageAreaVisibility`
  (if (`KismetStringLibrary.Contains` (`KismetSystemLibrary.GetDisplayName` (`.HitActor` (`GameplayStatics.BreakHitResult` (`PlayerController.GetHitResultUnderCursorByChannel` (`GameplayStatics.GetPlayerController` 0) "TraceTypeQuery1" true)))) "ExplosiveBarrel")
    (`SceneComponent.SetVisibility` (`self.DamageArea`) true false)
    (else
      (`SceneComponent.SetVisibility` (`self.DamageArea`) false false))))

(fn `UserConstructionScript`)