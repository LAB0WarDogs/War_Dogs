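; BP_Trap is a trap actor that paralyses an AI character that steps into its box.
; An AI overlap calls Paralysed on its controller, starts the player's trap skill cooldown, clears the trap-set flag and destroys the trap.
; The player's overlap only toggles the widget, while Interact cancels the trap skill and removes the trap.
; The player reference is found by class on BeginPlay.
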(event `self.Box.OnComponentBeginOverlap`
  (params (OverlappedComponent :type "PrimitiveComponent Object Reference") (OtherActor :type "Actor Object Reference") (OtherComp :type "PrimitiveComponent Object Reference") (OtherBodyIndex :type Integer) (bFromSweep :type Boolean) (SweepResult :type "HitResult Structure (by ref)"))
  (bind _bp_trap (`/Game/Blueprint/Character/BP_ThirdChara.BP_Trap` (`self.ThirdCharaRef`)))
  (cast `/Game/Blueprint/Character/BP_ThirdChara` OtherActor
    (:`then`
      (`SceneComponent.SetVisibility` (`self.Widget`) true false))
    (:`CastFailed`
      (bind _asbp_ai_master (cast `/Game/Blueprint/AI/AI_Puces/AiCharacter/BP_AI_Master` OtherActor))
      (bind _asbp_ai_controller_master (cast `/Game/Blueprint/AI/AI_Puces/AIController/BP_AiControllerMaster` (`AIBlueprintHelperLibrary.GetAIController` _asbp_ai_master)))
      (`/Game/Blueprint/AI/AI_Puces/AIController/BP_AiControllerMaster.Paralysed` _asbp_ai_controller_master 5.0 (`/Game/Blueprint/AI/AI_Puces/AIController/BP_AiControllerMaster.BTAsset` _asbp_ai_controller_master))
      (`/Game/Blueprint/SkiilsActorComponent/BP_TrapSkills.CoolDown` _bp_trap)
      (set `/Game/Blueprint/SkiilsActorComponent/BP_TrapSkills.TrapHasBeenSet` false _bp_trap)
      (`self.K2_DestroyActor`))))

(event `self.Box.OnComponentEndOverlap`
  (params (OverlappedComponent :type "PrimitiveComponent Object Reference") (OtherActor :type "Actor Object Reference") (OtherComp :type "PrimitiveComponent Object Reference") (OtherBodyIndex :type Integer))
  (cast `/Game/Blueprint/Character/BP_ThirdChara` OtherActor)
  (`SceneComponent.SetVisibility` (`self.Widget`) false false))

(event `/Game/Blueprint/Interface/BPI_InteractInterface.Interact`
  (bind _bp_trap (`/Game/Blueprint/Character/BP_ThirdChara.BP_Trap` (`self.ThirdCharaRef`)))
  (set `/Game/Blueprint/SkiilsActorComponent/BP_TrapSkills.TrapHasBeenSet` false _bp_trap)
  (`/Game/Blueprint/SkiilsActorComponent/BP_TrapSkills.CancelTrapSkill` _bp_trap)
  (`self.K2_DestroyActor`))

(event `self.ReceiveBeginPlay`
  (bind _returnvalue (`GameplayStatics.GetActorOfClass` "/Game/Blueprint/Character/BP_ThirdChara.BP_ThirdChara_C"))
  (set `self.ThirdCharaRef` _returnvalue))

(fn `UserConstructionScript`)