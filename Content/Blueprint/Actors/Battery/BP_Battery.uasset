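; BP_Battery is a battery pickup actor that the player collects through an Interact event.
; An overlap box shows a widget while a CharacterMaster is inside and hides it on exit.
; Interact checks the first player's battery count against its maximum, then calls AddBatteryToInventory and destroys the actor after a short delay.
; At maximum capacity, the battery stays in place.
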(event `/Game/Blueprint/Interface/BPI_InteractInterface.Interact`
  ;[0 0 1] Comment
  (bind _ascharacter_master (cast `/Game/Blueprint/Character/CharacterMaster` (`GameplayStatics.GetPlayerCharacter` 0)))
  (if (< (`/Game/Blueprint/Character/CharacterMaster.Battery` _ascharacter_master) (`/Game/Blueprint/Character/CharacterMaster.MaximumNumberOfBattery` _ascharacter_master))
    (`self.AddBatteryToInventory`)
    (`KismetSystemLibrary.Delay` 0.1)
    (`self.K2_DestroyActor`)))

(event `self.Box.OnComponentBeginOverlap`
  (params (OverlappedComponent :type "PrimitiveComponent Object Reference") (OtherActor :type "Actor Object Reference") (OtherComp :type "PrimitiveComponent Object Reference") (OtherBodyIndex :type Integer) (bFromSweep :type Boolean) (SweepResult :type "HitResult Structure (by ref)"))
  (cast `/Game/Blueprint/Character/CharacterMaster` OtherActor)
  (`SceneComponent.SetVisibility` (`self.Widget`) true false))

(event `self.Box.OnComponentEndOverlap`
  (params (OverlappedComponent :type "PrimitiveComponent Object Reference") (OtherActor :type "Actor Object Reference") (OtherComp :type "PrimitiveComponent Object Reference") (OtherBodyIndex :type Integer))
  (cast `/Game/Blueprint/Character/CharacterMaster` OtherActor)
  (`SceneComponent.SetVisibility` (`self.Widget`) false false))

(fn `UserConstructionScript`)