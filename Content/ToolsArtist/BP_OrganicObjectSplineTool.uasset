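; Artist spline tool that repeats a chosen mesh as deformed spline mesh segments along a spline.
; The construction script divides the spline by a section length, optionally derived from actor X scale, with an option to omit the partial end piece.
; Each segment takes local positions and tangents at its section boundaries, clamping tangents to section length.
; Segments use configurable collision and block the Visibility channel.
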(fn `GetEndPos/Tangent`
  (params (Index :type Integer))
  (returns (Pos :type "Vector Structure") (Tangent :type "Vector Structure"))
  (bind _spline (`self.Spline`))
  (bind _returnvalue (* (+ Index 1) (`self.SectionLenght`)))
  (return (`SplineComponent.GetLocationAtDistanceAlongSpline` _spline _returnvalue "Local") (`KismetMathLibrary.ClampVectorSize` (`SplineComponent.GetTangentAtDistanceAlongSpline` _spline _returnvalue "Local") 0.0 (`self.SectionLenght`))))

(fn `GetStartPos/Tangent`
  (params (Index :type Integer))
  (returns (Pos :type "Vector Structure") (Tangent :type "Vector Structure"))
  (bind _spline (`self.Spline`))
  (bind _returnvalue (* Index (`self.SectionLenght`)))
  (return (`SplineComponent.GetLocationAtDistanceAlongSpline` _spline _returnvalue "Local") (`KismetMathLibrary.ClampVectorSize` (`SplineComponent.GetTangentAtDistanceAlongSpline` _spline _returnvalue "Local") 0.0 (`self.SectionLenght`))))

(fn `UserConstructionScript`
  (locals (NumberOfInstances :type Integer :default 0))
  (bind _returnvalue_x (`KismetMathLibrary.BreakVector` (`self.GetActorScale3D`)))
  (if (`self.AllowScaling`)
    ;[1 1 1] Scale the spline ?
    (set `self.SectionLenght` (* _returnvalue_x 100.0)))
  (if (`self.MustBeFullLenghtMeshes`)
    ;[1 1 1] remove half pieces at end of spline => Meshes must be full lenght to be spawned
    (for _index (range (`KismetMathLibrary.FTrunc` (/ (`SplineComponent.GetSplineLength` (`self.Spline`)) (`self.SectionLenght`))))
      (set `self.LoopIndex` _index)
      (bind _returnvalue (`AddComponent|NODE_AddSplineMeshComponent-1` :!label _label))
      (`StaticMeshComponent.SetStaticMesh` _returnvalue (`self.PlacedMesh`))
      (`SplineMeshComponent.SetForwardAxis` _returnvalue (`self.MeshAxis`) true)
      (bind (_pos _tangent) (`self.GetStartPos/Tangent` (`self.LoopIndex`)))
      (bind (_pos_2 _tangent_2) (`self.GetEndPos/Tangent` (`self.LoopIndex`)))
      (`SplineMeshComponent.SetStartAndEnd` _returnvalue _pos _tangent _pos_2 _tangent_2 true)
      (`PrimitiveComponent.SetCollisionEnabled` _returnvalue (`self.CollisionType`))
      (`PrimitiveComponent.SetCollisionResponseToChannel` _returnvalue "ECC_Visibility" "ECR_Block"))
    (else
      ;[1 1 1] Spline lenght divide by section lenght = Amount of spline meshes
      (for _index_2 (range (+ (`KismetMathLibrary.FTrunc` (/ (`SplineComponent.GetSplineLength` (`self.Spline`)) (`self.SectionLenght`))) 1))
        (set `self.LoopIndex` _index_2)
        (goto _label)))))